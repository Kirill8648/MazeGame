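; Gameplay ability that raises the maze walls around the hero, with a delay that grows with distance so they lift in an outward ripple.
; On activation it caches the hero and ASC, reads level-based radius and air time from a stats table, then sphere-overlaps from the first-person camera.
; Instanced mesh walls in range are swapped for actors and raised like existing wall actors.
; It also draws a debug sphere of the radius.
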(event `self.K2_ActivateAbility`
  (bind _abilityslotref (`self.AbilitySlotRef`))
  (bind _radiuscache (`self.RadiusCache`))
  (bind _returnvalue (`SceneComponent.K2_GetComponentLocation` (`MGHeroCharacter.FirstPersonCamera` (`self.OwningHero`))))
  (bind _returnvalue_2 (`SceneComponent.K2_GetComponentLocation` (`MGHeroCharacter.FirstPersonCamera` (`self.OwningHero`))))
  (`UserWidget.PlayAnimation` _abilityslotref (`/Game/MazeGame/UI/Widgets/HUD/WBP_HUDAbilitySlot.ActivatingOnce` _abilityslotref) 0.0 1 "Forward" 1.0 false)
  (`self.CheckAndSetupCacheables`)
  (`self.K2_CommitAbility`)
  (`KismetSystemLibrary.DrawDebugSphere` _returnvalue _radiuscache 16 (struct :`R` 1.0 :`B` 0.016776 :`A` 1.0) 5.0 5.0)
  (bind _outactors (`KismetSystemLibrary.SphereOverlapActors` _returnvalue _radiuscache (`|MakeArray` "ObjectTypeQuery1" "ObjectTypeQuery2" :!type "EObjectTypeQuery Enum") "/Script/Engine.Actor"))
  (for _array_element _outactors
    (bind _asmginstanced_mesh_actor (cast `MGInstancedMeshActor` _array_element)
      (:`then`
        (bind _returnvalue_3 (`MGInstancedMeshActor.ReplaceInstancesWithActorsBySphereOverlap` _asmginstanced_mesh_actor _returnvalue_2 (`self.RadiusCache`)))
        (for _array_element_2 _returnvalue_3
          (bind _asbp_maze_wall_base (cast `/Game/MazeGame/Maze/Walls/BP_MazeWallBase` _array_element_2))
          (set `/Game/MazeGame/Maze/Walls/BP_MazeWallBase.TimeInAir` (`self.TimeInAirCachr`) _asbp_maze_wall_base)
          (set `/Game/MazeGame/Maze/Walls/BP_MazeWallBase.DelayBeforeRaise` (`KismetMathLibrary.NormalizeToRange` (`KismetMathLibrary.Vector_Distance` (`Actor.K2_GetActorLocation` _asbp_maze_wall_base) _returnvalue_2) 175.0 (* (`self.RadiusCache`) 1.0)) _asbp_maze_wall_base)
          (`/Game/MazeGame/Maze/Walls/BP_MazeWallBase.Raise` _asbp_maze_wall_base)))
      (:`CastFailed`
        (bind _asbp_maze_wall_base_2 (cast `/Game/MazeGame/Maze/Walls/BP_MazeWallBase` _array_element))
        (set `/Game/MazeGame/Maze/Walls/BP_MazeWallBase.TimeInAir` (`self.TimeInAirCachr`) _asbp_maze_wall_base_2)
        (set `/Game/MazeGame/Maze/Walls/BP_MazeWallBase.DelayBeforeRaise` (`KismetMathLibrary.NormalizeToRange` (`KismetMathLibrary.Vector_Distance` (`Actor.K2_GetActorLocation` _asbp_maze_wall_base_2) (`SceneComponent.K2_GetComponentLocation` (`MGHeroCharacter.FirstPersonCamera` (`self.OwningHero`)))) 175.0 (* (`self.RadiusCache`) 1.0)) _asbp_maze_wall_base_2)
        (`/Game/MazeGame/Maze/Walls/BP_MazeWallBase.Raise` _asbp_maze_wall_base_2))))
  (`self.K2_EndAbility`))

(event `self.K2_OnEndAbility`
  (params (bWasCancelled :type Boolean)))