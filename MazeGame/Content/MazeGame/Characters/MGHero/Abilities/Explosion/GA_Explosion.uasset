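; Hero gameplay ability for a hold-to-charge explosion that wrecks maze walls around the first-person camera.
; Radius and hold time come from a per-level stats table, with a radius visual, indicator and cancel hint shown while charging.
; Release or timeout scales a sphere trace, camera shake and radial field by charge, replacing near walls and physics-simulating far ones.
; Charge above 90% applies self-damage scaled to max health, up to all of it.
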(event `self.K2_ActivateAbility`
  (bind _asc (`self.ASC`))
  (bind _abilityslotref (`self.AbilitySlotRef`))
  (bind _returnvalue (`SceneComponent.K2_GetComponentLocation` (`MGHeroCharacter.FirstPersonCamera` (`self.OwningHero`))))
  (`UserWidget.PlayAnimation` _abilityslotref (`/Game/MazeGame/UI/Widgets/HUD/WBP_HUDAbilitySlot.ActivatingFadeIn` _abilityslotref) 0.0 1 "Forward" 1.0 false)
  (`self.CheckAndSetupCacheables`)
  (`self.CreateVisuals`)
  (bind (_asynctaskproxy _timeheld) (`AbilityTask_WaitInputRelease.WaitInputRelease` true)
    (:`then`
      (set `self.WaitReleaseTask` _asynctaskproxy)
      (bind _asynctaskproxy_2 (`AbilityTask_WaitDelay.WaitDelay` (`self.MaxHoldTime`))
        (:`then`
          (set `self.WaitDelayTask` _asynctaskproxy_2)
          (bind _asynctaskproxy_3 (`AbilityTask_WaitCancel.WaitCancel`)
            (:`then`
              (set `self.WaitCancelInputTask` _asynctaskproxy_3))
            (:`OnCancel`
              (`self.K2_CancelAbility`))))
        (:`OnFinish`
          (set `self.bIsFinishedByDelay` true)
          (`self.K2_CommitAbilityCost` false :!label _label)
          (bind _returnvalue_2 (select `bool` (`self.bIsFinishedByDelay`) :`false` (/ _timeheld (`self.MaxHoldTime`)) :`true` 1.0))
          (`PlayerCameraManager.StartCameraShake` :`self` (`GameplayStatics.GetPlayerCameraManager` 0) :`ShakeClass` "/Game/MazeGame/Characters/MGHero/Abilities/Explosion/ExplosionShake.ExplosionShake_C" :`Scale` _returnvalue_2)
          (bind _returnvalue_3 (* _returnvalue_2 (`self.MaxRadiusCache`)))
          (bind _outhits (`KismetSystemLibrary.SphereTraceMultiForObjects` _returnvalue _returnvalue _returnvalue_3 (`|MakeArray` "ObjectTypeQuery1" "ObjectTypeQuery2" :!type "EObjectTypeQuery Enum") false (`|MakeArray` (`GameplayStatics.GetPlayerCharacter` 0) :!type "Actor Object Reference") "ForDuration"))
          (for _array_element _outhits
            (bind _asbp_maze_wall_base (cast `/Game/MazeGame/Maze/Walls/BP_MazeWallBase` (`.HitActor` (`GameplayStatics.BreakHitResult` _array_element))))
            (if (> (`KismetMathLibrary.Vector_Distance` (`Actor.K2_GetActorLocation` _asbp_maze_wall_base) (`SceneComponent.K2_GetComponentLocation` (`MGHeroCharacter.FirstPersonCamera` (`self.OwningHero`)))) 1500.0)
              (`PrimitiveComponent.SetSimulatePhysics` (`/Game/MazeGame/Maze/Walls/BP_MazeWallBase.WallSimpleMesh` _asbp_maze_wall_base) true)
              (`Actor.SetLifeSpan` _asbp_maze_wall_base 5.0)
              (else
                (`/Game/MazeGame/Maze/Walls/BP_MazeWallBase.Destroy(Replace)` _asbp_maze_wall_base 5.0))))
          (bind _returnvalue_4 (- _returnvalue_2 0.9))
          (bind _returnvalue_5 (`AbilitySystemBlueprintLibrary.AssignTagSetByCallerMagnitude` (`AbilitySystemComponent.MakeOutgoingSpec` :`self` _asc :`GameplayEffectClass` "/Game/MazeGame/Characters/MGHero/GamepalyEffects/GE_InstantDamageSetByCaller.GE_InstantDamageSetByCaller_C" :`Level` 1.0) (struct :`TagName` "SetByCaller.Damage") (`KismetMathLibrary.Conv_IntToDouble` (`KismetMathLibrary.Round` (select `bool` (> _returnvalue_4 0.0) :`true` (* (* _returnvalue_4 10.0) (`MGCharacterBase.GetMaxHealth` (`self.OwningHero`)) -1.0))))))
          (`AbilitySystemComponent.BP_ApplyGameplayEffectSpecToSelf` _asc _returnvalue_5)
          (bind _returnvalue_6 (`|SpawnActorFromClass` "/Game/MazeGame/Characters/MGHero/Abilities/FS_MGSphereField.FS_MGSphereField_C" (`KismetMathLibrary.MakeTransform` (`SceneComponent.K2_GetComponentLocation` (`MGHeroCharacter.FirstPersonCamera` (`self.OwningHero`)))) "Undefined" "OverrideRootScale" null null))
          (`SphereComponent.SetSphereRadius` (`/Engine/EditorResources/FieldNodes/FS_MasterField.SphereVolumeCol` _returnvalue_6) _returnvalue_3 false)
          (set `/Engine/EditorResources/FieldNodes/FS_MasterField.Radial Magnitude` (/ _returnvalue_3 4.0) _returnvalue_6)
          (`Actor.SetLifeSpan` _returnvalue_6 0.5)
          (`self.K2_CommitAbilityCooldown` false)
          (`self.K2_EndAbility`))))
    (:`OnRelease`
      (goto _label))))

(event `self.K2_OnEndAbility`
  (params (bWasCancelled :type Boolean))
  (bind _abilityslotref (`self.AbilitySlotRef`))
  (`GameplayTask.EndTask` (`self.WaitReleaseTask`))
  (`GameplayTask.EndTask` (`self.WaitCancelInputTask`))
  (`GameplayTask.EndTask` (`self.WaitDelayTask`))
  (`UserWidget.PlayAnimation` _abilityslotref (`/Game/MazeGame/UI/Widgets/HUD/WBP_HUDAbilitySlot.ActivatingFadeOut` _abilityslotref) 0.0 1 "Forward" 1.0 false)
  (`Widget.RemoveFromParent` (`self.IndicatorWidgetRef`))
  (`PanelWidget.RemoveChild` (`/Game/MazeGame/UI/Widgets/HUD/WBP_HUDProgressBars.HintsBox` (`/Game/MazeGame/UI/BP_MGHUD.ProgressBarsWidget` (`self.As BP MGHUD`))) (`self.HintWidgetRef`))
  (`Actor.K2_DestroyActor` (`self.VisualActorRef`)))