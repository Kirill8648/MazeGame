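; Visual actor for the hero's explosion ability that shows the radius as an expanding sphere.
; On BeginPlay it starts a timer and opens a Gate, letting Tick scale the sphere from the timer's elapsed time toward MaxRadius over OverTime.
; Each update also moves the sphere to the character's first-person camera.
; When the timer ends, updates stop; the actor does not destroy itself here.
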(event `self.ReceiveBeginPlay`
  (`self.Start`))

(event `self.ReceiveTick`
  (params (DeltaSeconds :type "Float (single-precision)"))
  (bind _sphere (`self.Sphere`))
  (`/Engine/EditorBlueprintResources/StandardMacros.Gate` true :!label _label
    (:`Exit`
      (`SceneComponent.SetRelativeScale3D` _sphere (`KismetMathLibrary.Conv_DoubleToVector` (/ (`KismetMathLibrary.MapRangeClamped` (`KismetSystemLibrary.K2_GetTimerElapsedTimeHandle` (stale `Start` _output_get)) 0.0 (`self.OverTime`) 0.0 (`self.MaxRadius`)) 1000.0)))
      (`SceneComponent.K2_SetWorldLocation` _sphere (`SceneComponent.K2_GetComponentLocation` (`MGHeroCharacter.FirstPersonCamera` (`self.CharRef`))) false false))))

(event `Finished`
  (`KismetSystemLibrary.K2_ClearAndInvalidateTimerHandle` (`self.TimerHandle`))
  (goto _label :!via `Close`))

(event `Start`
  (bind _returnvalue (`KismetSystemLibrary.K2_SetTimerDelegate` (delegate `Finished`) (`self.OverTime`)))
  (bind _output_get (set `self.TimerHandle` _returnvalue))
  (goto _label :!via `Open`))

(fn `UserConstructionScript`)