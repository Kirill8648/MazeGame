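; GA_Vision is the hero's timed vision ability, highlighting abilities, traps and boosters through camera post-processing.
; It reads level-based distance and duration from StatsTable, sets the view distance, alters camera tone-mapping and enables more custom-stencil highlight channels at each of three levels.
; It ends on timeout or another press of its input, shown in a HUD hint, then commits cooldown and reverts the effect.
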(event `self.K2_ActivateAbility`
  (bind _abilityslotref (`self.AbilitySlotRef`))
  (bind _owninghero (`self.OwningHero`))
  (bind _fpscamerapp (`/Game/MazeGame/Characters/MGHero/BP_MGHeroCharacter.FPSCameraPP` (`self.OwningHero`)))
  (bind ((`FilmSlope` _filmslope) (`FilmToe` _filmtoe) (`FilmShoulder` _filmshoulder) (`FilmBlackClip` _filmblackclip)) (break `PostProcessSettings` (`CameraComponent.PostProcessSettings` (`MGHeroCharacter.FirstPersonCamera` _owninghero))))
  (`self.CheckAndSetupCacheables`)
  (`UserWidget.PlayAnimation` _abilityslotref (`/Game/MazeGame/UI/Widgets/HUD/WBP_HUDAbilitySlot.ActivatingFadeIn` _abilityslotref) 0.0 1 "Forward" 1.0 false)
  (`self.K2_CommitAbilityCost` false)
  (bind _returnvalue (`|CreateWidget` "/Game/MazeGame/UI/Widgets/HUD/WBP_HintText.WBP_HintText_C"))
  (bind _output_get (set `self.HintWidgetRef` _returnvalue))
  (`RichTextBlock.SetText` (`/Game/MazeGame/UI/Widgets/HUD/WBP_HintText.RichTextBlock` _output_get) (`KismetTextLibrary.Conv_StringToText` (`KismetStringLibrary.Concat_StrStr` "<Outlined>" (`KismetTextLibrary.Conv_TextToString` (`KismetInputLibrary.Key_GetDisplayName` (`.Key` (break `InputActionKeyMapping` (`|GetArrayItem` (`InputSettings.GetActionMappingByName` (`InputSettings.GetInputSettings`) (`KismetStringLibrary.Conv_StringToName` (`|GetEnumeratorNameAsString` (`self.AbilityInputID`))))))))) "</>" "<OutlinedLight>" (`KismetTextLibrary.Conv_TextToString` " - Turn off vision") "</>")))
  (bind _returnvalue_2 (`VerticalBox.AddChildToVerticalBox` (`/Game/MazeGame/UI/Widgets/HUD/WBP_HUDProgressBars.HintsBox` (`/Game/MazeGame/UI/BP_MGHUD.ProgressBarsWidget` (`self.As BP MGHUD`))) (`self.HintWidgetRef`)))
  (`VerticalBoxSlot.SetPadding` _returnvalue_2 (make `Margin` 0.0 5.0 0.0 5.0))
  (`MaterialInstanceDynamic.SetScalarParameterValue` (`/Game/MazeGame/Characters/MGHero/BP_MGHeroCharacter.FPSCameraPP` _owninghero) "ViewDistance" (`self.Distance`))
  (`|VariableSetRef` _filmslope 0.2)
  (`|VariableSetRef` _filmtoe 0.3)
  (`|VariableSetRef` _filmblackclip 0.35)
  (switch `int` (`self.GetAbilityLevel`)
    (:`Default`
      (`KismetSystemLibrary.PrintString` "Not Correct level in GA_Vision" true true (struct :`R` 1.0 :`A` 1.0) 10.0))
    (:`1`
      ;[1 1 1] Highlights Abilities
      (`MaterialInstanceDynamic.SetScalarParameterValue` _fpscamerapp "RenderStencil3" 1.0)
      (bind _asynctaskproxy (`AbilityTask_WaitDelay.WaitDelay` (`self.Duration`) :!label _label)
        (:`then`
          (set `self.DelayTask` _asynctaskproxy)
          (bind _asynctaskproxy_2 (`AbilityTask_WaitInputPress.WaitInputPress` false)
            (:`then`
              (set `self.InputPressTask` _asynctaskproxy_2))
            (:`OnPress`
              (`self.K2_EndAbility`))))
        (:`OnFinish`
          (`self.K2_EndAbility`))))
    (:`2`
      ;[1 1 1] Highlights Abilities and Deadly Traps
      (`MaterialInstanceDynamic.SetScalarParameterValue` _fpscamerapp "RenderStencil2" 1.0)
      (`MaterialInstanceDynamic.SetScalarParameterValue` _fpscamerapp "RenderStencil3" 1.0)
      (goto _label))
    (:`3`
      ;[1 1 1] Highlights Abilities, Important Boosters and All Traps
      (`MaterialInstanceDynamic.SetScalarParameterValue` _fpscamerapp "RenderStencil1" 1.0)
      (`MaterialInstanceDynamic.SetScalarParameterValue` _fpscamerapp "RenderStencil2" 1.0)
      (`MaterialInstanceDynamic.SetScalarParameterValue` _fpscamerapp "RenderStencil3" 1.0)
      (`MaterialInstanceDynamic.SetScalarParameterValue` _fpscamerapp "RenderStencil4" 1.0)
      (goto _label))))

(event `self.K2_OnEndAbility`
  (params (bWasCancelled :type Boolean))
  (bind _owninghero (`self.OwningHero`))
  (bind _abilityslotref (`self.AbilitySlotRef`))
  (bind _fpscamerapp (`/Game/MazeGame/Characters/MGHero/BP_MGHeroCharacter.FPSCameraPP` _owninghero))
  (bind ((`FilmSlope` _filmslope) (`FilmToe` _filmtoe) (`FilmShoulder` _filmshoulder) (`FilmBlackClip` _filmblackclip)) (break `PostProcessSettings` (`CameraComponent.PostProcessSettings` (`MGHeroCharacter.FirstPersonCamera` _owninghero))))
  (`self.K2_CommitAbilityCooldown` false)
  (`UserWidget.PlayAnimation` _abilityslotref (`/Game/MazeGame/UI/Widgets/HUD/WBP_HUDAbilitySlot.ActivatingFadeOut` _abilityslotref) 0.0 1 "Forward" 1.0 false)
  (`GameplayTask.EndTask` (`self.DelayTask`))
  (`GameplayTask.EndTask` (`self.InputPressTask`))
  (`|VariableSetRef` _filmslope 0.88)
  (`|VariableSetRef` _filmtoe 0.55)
  (`|VariableSetRef` _filmblackclip)
  (`MaterialInstanceDynamic.SetScalarParameterValue` _fpscamerapp "ViewDistance" 0.0)
  (`MaterialInstanceDynamic.SetScalarParameterValue` _fpscamerapp "RenderStencil1" 0.0)
  (`MaterialInstanceDynamic.SetScalarParameterValue` _fpscamerapp "RenderStencil2" 0.0)
  (`MaterialInstanceDynamic.SetScalarParameterValue` _fpscamerapp "RenderStencil3" 0.0)
  (`MaterialInstanceDynamic.SetScalarParameterValue` _fpscamerapp "RenderStencil3" 0.0)
  (`Widget.RemoveFromParent` (`self.HintWidgetRef`)))