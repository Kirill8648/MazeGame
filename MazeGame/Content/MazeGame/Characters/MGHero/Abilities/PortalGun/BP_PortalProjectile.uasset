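; BP_PortalProjectile is the shot of the portal gun ability, placing a portal where it hits.
; On impact, a portal-sized box trace just off the surface checks for clearance: if blocked it ends GAPortalGun, otherwise it has the ability respawn the portal there.
; It then spawns a tinted Niagara burst and destroys itself.
; The construction script applies its material and initial speed.
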(event `self.Sphere.OnComponentHit`
  (params (HitComponent :type "PrimitiveComponent Object Reference") (OtherActor :type "Actor Object Reference") (OtherComp :type "PrimitiveComponent Object Reference") (NormalImpulse :type "Vector Structure") (Hit :type "HitResult Structure (by ref)"))
  (bind (_bblockinghit _binitialoverlap _time _distance _location _impactpoint _normal) (`GameplayStatics.BreakHitResult` Hit))
  (bind _ga_portalgun (`self.GA_PortalGun`))
  (bind _returnvalue (* _normal 15.0))
  (bind _returnvalue_2 (+ _impactpoint _returnvalue))
  (bind _returnvalue_3 (`KismetMathLibrary.FindLookAtRotation` _impactpoint (+ (`SceneComponent.K2_GetComponentLocation` (`self.Sphere`)) _returnvalue)))
  (bind (_outhit _returnvalue_4) (`KismetSystemLibrary.BoxTraceSingle` :`Start` _returnvalue_2 :`End` _returnvalue_2 :`HalfSize` (12.0 62.0 112.0) :`Orientation` _returnvalue_3 :`TraceChannel` "TraceTypeQuery1" :`DrawDebugType` "ForDuration" :`DrawTime` 1.0))
  (set `PrimitiveComponent.bGenerateOverlapEvents` false (`self.Sphere`))
  (if _returnvalue_4
    (`GameplayAbility.K2_EndAbility` _ga_portalgun)
    (else
      (`/Game/MazeGame/Characters/MGHero/Abilities/PortalGun/GA_PortalGun1.(Re) Spawn Portal` _ga_portalgun (+ _impactpoint (* _normal 25.0)) _returnvalue_3)))
  (bind _returnvalue_5 (`NiagaraFunctionLibrary.SpawnSystemAtLocation` "/Game/MazeGame/Characters/MGHero/Abilities/PortalGun/NS_Burst.NS_Burst" _location))
  (`NiagaraComponent.SetVariableLinearColor` _returnvalue_5 "Color" (`self.ParticleColor`))
  (`self.K2_DestroyActor`))

(fn `UserConstructionScript`
  (`PrimitiveComponent.SetMaterial` (`self.Sphere`) 0 (`self.MI`))
  (set `ProjectileMovementComponent.InitialSpeed` (`self.Speed`) (`self.ProjectileMovement`)))