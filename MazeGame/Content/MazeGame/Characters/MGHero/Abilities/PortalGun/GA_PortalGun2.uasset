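; GA_PortalGun2 is a portal gun gameplay ability whose function replaces its BP_PortalMaster_Portal1 at a given location and rotation.
; It destroys the previous portal, spawns a new one and assigns CRT_FirstPortal as its cube scene capture target.
; It cross-links the new portal with the first BP_PortalMaster found, refreshes that portal's capture, then commits and ends the ability.
; The activation and end events here are disabled stubs.
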(fn `(Re) Spawn Portal`
  (params (Location :type "Vector Structure") (Rotation :type "Rotator Structure"))
  (bind _spawnedportal (`self.SpawnedPortal`))
  (bind _anotherportal (`self.AnotherPortal`))
  (bind _spawnedportal_2 (`self.SpawnedPortal`)
    (:`then`
      (`Actor.K2_DestroyActor` _spawnedportal_2))
    (:`else`
      _))
  (bind _outactors (`GameplayStatics.GetAllActorsOfClass` "/Game/MazeGame/Characters/MGHero/Abilities/PortalGun/BP_PortalMaster.BP_PortalMaster_C"))
  (set `self.AnotherPortal` (`|GetArrayItem` _outactors))
  (bind _returnvalue (`|SpawnActorFromClass` "/Game/MazeGame/Characters/MGHero/Abilities/PortalGun/BP_PortalMaster_Portal1.BP_PortalMaster_Portal1_C" (`KismetMathLibrary.MakeTransform` Location Rotation) "Undefined" "OverrideRootScale" null (`self.MI`) null))
  (bind _output_get (set `self.SpawnedPortal` _returnvalue))
  (set `SceneCaptureComponentCube.TextureTarget` "/Game/MazeGame/Characters/MGHero/Abilities/PortalGun/CRT_FirstPortal.CRT_FirstPortal" (`/Game/MazeGame/Characters/MGHero/Abilities/PortalGun/BP_PortalMaster.SceneCaptureComponentCube` _output_get))
  (`/Engine/EditorBlueprintResources/StandardMacros.IsValid` _anotherportal
    (:`Is Valid`
      (`/Game/MazeGame/Characters/MGHero/Abilities/PortalGun/BP_PortalMaster.AddAnother` _anotherportal _spawnedportal)
      (`/Game/MazeGame/Characters/MGHero/Abilities/PortalGun/BP_PortalMaster.AddAnother` _spawnedportal _anotherportal)
      (`SceneCaptureComponentCube.CaptureScene` (`/Game/MazeGame/Characters/MGHero/Abilities/PortalGun/BP_PortalMaster.SceneCaptureComponentCube` (`self.AnotherPortal`))))
    (:`Is Not Valid`
      _))
  (`self.K2_CommitAbility`)
  (`self.K2_EndAbility`))