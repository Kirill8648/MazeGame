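; Gameplay ability for the hero's portal gun that fires and places Portal1.
; Activation fires a projectile from the first-person camera at a level-based speed from a data table; another press cancels it.
; The projectile receives the ability reference, and ReSpawnPortal replaces the previous portal, linking it with another found portal for scene-capture views.
; The ability commits only when a portal spawns, so cancelled shots skip the commit.
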(event `self.K2_ActivateAbility`
  (bind _abilityslotref (`self.AbilitySlotRef`))
  (bind _firstpersoncamera (`MGHeroCharacter.FirstPersonCamera` (`self.OwningHero`)))
  (`self.CheckAndSetupCacheables`)
  (`UserWidget.PlayAnimation` _abilityslotref (`/Game/MazeGame/UI/Widgets/HUD/WBP_HUDAbilitySlot.ActivatingOnce` _abilityslotref) 0.0 1 "Forward" 1.0 false)
  (bind _returnvalue (`|SpawnActorFromClass` "/Game/MazeGame/Characters/MGHero/Abilities/PortalGun/BP_PortalProjectile.BP_PortalProjectile_C" (`KismetMathLibrary.MakeTransform` (+ (`SceneComponent.K2_GetComponentLocation` _firstpersoncamera) (* (`SceneComponent.GetForwardVector` _firstpersoncamera) 1.0)) (`SceneComponent.K2_GetComponentRotation` _firstpersoncamera)) "Undefined" "OverrideRootScale" null (`self.MI`) self (`self.ShootSpeed`) (`self.ParticleColor`) null))
  (`AbilityTask_WaitInputPress.WaitInputPress` false
    (:`OnPress`
      (`Actor.K2_DestroyActor` _returnvalue)
      (`self.K2_EndAbility`))))

(event `self.K2_OnEndAbility`
  (params (bWasCancelled :type Boolean)))

(fn `(Re) Spawn Portal`
  (params (Location :type "Vector Structure") (Rotation :type "Rotator Structure"))
  (bind _spawnedportal (`self.SpawnedPortal`))
  (bind _anotherportal (`self.AnotherPortal`))
  (bind _spawnedportal_2 (`self.SpawnedPortal`)
    (:`then`
      (`Actor.K2_DestroyActor` _spawnedportal_2))
    (:`else`
      _))
  (bind _outactors (`GameplayStatics.GetAllActorsOfClass` "/Game/MazeGame/Characters/MGHero/Abilities/PortalGun/BP_PortalMaster.BP_PortalMaster_C"))
  (set `self.AnotherPortal` (`|GetArrayItem` _outactors))
  (bind _returnvalue (`|SpawnActorFromClass` "/Game/MazeGame/Characters/MGHero/Abilities/PortalGun/BP_PortalMaster_Portal1.BP_PortalMaster_Portal1_C" (`KismetMathLibrary.MakeTransform` Location Rotation) "Undefined" "OverrideRootScale" null (`self.MI`) null))
  (bind _output_get (set `self.SpawnedPortal` _returnvalue))
  (set `SceneCaptureComponentCube.TextureTarget` "/Game/MazeGame/Characters/MGHero/Abilities/PortalGun/CRT_SecondPortal.CRT_SecondPortal" (`/Game/MazeGame/Characters/MGHero/Abilities/PortalGun/BP_PortalMaster.SceneCaptureComponentCube` _output_get))
  (`/Engine/EditorBlueprintResources/StandardMacros.IsValid` _anotherportal
    (:`Is Valid`
      (`/Game/MazeGame/Characters/MGHero/Abilities/PortalGun/BP_PortalMaster.AddAnother` _anotherportal _spawnedportal)
      (`/Game/MazeGame/Characters/MGHero/Abilities/PortalGun/BP_PortalMaster.AddAnother` _spawnedportal _anotherportal)
      (`SceneCaptureComponentCube.CaptureScene` (`/Game/MazeGame/Characters/MGHero/Abilities/PortalGun/BP_PortalMaster.SceneCaptureComponentCube` (`self.AnotherPortal`))))
    (:`Is Not Valid`
      _))
  (`self.K2_CommitAbility`)
  (`self.K2_EndAbility`))