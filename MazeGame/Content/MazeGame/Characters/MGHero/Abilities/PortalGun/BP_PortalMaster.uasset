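; One end of a linked portal pair that teleports the hero and other actors to its partner.
; A cube scene capture, refreshed on a randomly offset timer or in real time per player settings, feeds the partner's dynamic Niagara material.
; Overlaps redirect velocity along the exit's forward vector with a minimum speed, including physics components and Scout projectiles.
; Exit portals are hidden or disabled until overlap ends, preventing bounce-back.
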(event `self.ReceiveBeginPlay`
  (bind _returnvalue (subsystem `MGPlayerDataSubsystem`))
  (bind _scenecapturecomponentcube (`self.SceneCaptureComponentCube`))
  (bind _brealtimeportals (`MGPlayerDataSubsystem.bRealTimePortals` _returnvalue))
  (`KismetSystemLibrary.Delay` (`KismetMathLibrary.RandomFloatInRange` 0.0 1.0))
  (`KismetSystemLibrary.K2_SetTimerDelegate` (delegate `UpdateCapture`) (`MGPlayerDataSubsystem.PortalsUpdateRate` _returnvalue) true)
  (set `SceneCaptureComponent.bCaptureEveryFrame` _brealtimeportals _scenecapturecomponentcube)
  (set `SceneCaptureComponent.bCaptureOnMovement` _brealtimeportals _scenecapturecomponentcube))

(event `UpdateCapture`
  (if (`self.bIsOtherActive`)
    (`SceneCaptureComponentCube.CaptureScene` (`self.SceneCaptureComponentCube`))))

(event `AddAnother`
  (params (OtherPointer :type "/Game/MazeGame/Characters/MGHero/Abilities/PortalGun/BP_PortalMaster Object Reference"))
  (bind _materialinstdynamic (`self.MaterialInstDynamic`))
  (bind _output_get (set `self.OtherPointer` OtherPointer))
  (`MaterialInstanceDynamic.SetTextureParameterValue` _materialinstdynamic "CubeCapture" (`SceneCaptureComponentCube.TextureTarget` (`/Game/MazeGame/Characters/MGHero/Abilities/PortalGun/BP_PortalMaster.SceneCaptureComponentCube` _output_get)))
  (`MaterialInstanceDynamic.SetScalarParameterValue` _materialinstdynamic "bIsOtherPortalActive" 1.0)
  (set `self.bIsOtherActive` true)
  (`self.UpdateCubemapNormalVector`))

(event `RemoveAnother`
  (bind _materialinstdynamic (`self.MaterialInstDynamic`))
  (set `self.OtherPointer` null)
  (`MaterialInstanceDynamic.SetTextureParameterValue` _materialinstdynamic "CubeCapture" null)
  (`MaterialInstanceDynamic.SetScalarParameterValue` _materialinstdynamic "bIsOtherPortalActive" 0.0)
  (set `self.bIsOtherActive` false))

(event `self.Box.OnComponentBeginOverlap`
  (params (OverlappedComponent :type "PrimitiveComponent Object Reference") (OtherActor :type "Actor Object Reference") (OtherComp :type "PrimitiveComponent Object Reference") (OtherBodyIndex :type Integer) (bFromSweep :type Boolean) (SweepResult :type "HitResult Structure (by ref)"))
  (bind _otherpointer (`self.OtherPointer`))
  (bind _as_bp_mghero_character (`self.As BP MGHero Character`))
  (bind _rootcomponent (`Actor.RootComponent` OtherActor))
  (bind _otherpointer_2 (`self.OtherPointer`))
  (bind _charactermovement (`Character.CharacterMovement` _as_bp_mghero_character))
  (bind _ns_portal (`/Game/MazeGame/Characters/MGHero/Abilities/PortalGun/BP_PortalMaster.NS_Portal` _otherpointer))
  (if (and (`self.bCanPort`) (`self.bIsOtherActive`))
    (bind _asbp_mghero_character (cast `/Game/MazeGame/Characters/MGHero/BP_MGHeroCharacter` OtherActor)
      (:`then`
        (set `self.As BP MGHero Character` _asbp_mghero_character)
        (`self.Hide Self` _otherpointer_2)
        (`KismetSystemLibrary.Delay` 0.05)
        (`SceneComponent.K2_SetWorldLocation` (`Character.CapsuleComponent` _as_bp_mghero_character) (`SceneComponent.K2_GetComponentLocation` (`/Game/MazeGame/Characters/MGHero/Abilities/PortalGun/BP_PortalMaster.NS_Portal` _otherpointer_2)) false true)
        (set `MovementComponent.Velocity` (* (`self.GetActorForwardVector` (`self.OtherPointer`)) (`KismetMathLibrary.FClamp` (`KismetMathLibrary.VSize` (`CharacterMovementComponent.GetLastUpdateVelocity` _charactermovement)) 200.0 9999999.0)) _charactermovement))
      (:`CastFailed`
        (set `/Game/MazeGame/Characters/MGHero/Abilities/PortalGun/BP_PortalMaster.bCanPort` false _otherpointer)
        (`SceneComponent.K2_SetWorldLocation` _rootcomponent (+ (`SceneComponent.K2_GetComponentLocation` _ns_portal) (* (`SceneComponent.GetForwardVector` _ns_portal) 10.0)) false true)
        (`SceneComponent.K2_SetWorldRotation` _rootcomponent (`SceneComponent.K2_GetComponentRotation` _ns_portal) false true)
        (bind _asprimitive_component (cast `PrimitiveComponent` _rootcomponent)
          (:`then`
            (`MGAsyncTaskPCTempCollisionChange.TempCollisionChange` _asprimitive_component 0.5
              (:`then`
                (`self.SetVelocityToPrimitiveComponent` _asprimitive_component))))
          (:`CastFailed`
            _))
        (for _array_element (`SceneComponent.GetChildrenComponents` _rootcomponent true)
          (bind _asprimitive_component_2 (cast `PrimitiveComponent` _array_element))
          (`MGAsyncTaskPCTempCollisionChange.TempCollisionChange` _asprimitive_component_2 0.5
            (:`then`
              (`self.SetVelocityToPrimitiveComponent` _asprimitive_component_2))))
        (bind _asbp_scout_v2 (cast `/Game/MazeGame/Characters/MGHero/Abilities/ScoutLaunch/BP_ScoutV2` OtherActor))
        (bind _projectilemovement (`/Game/MazeGame/Characters/MGHero/Abilities/ScoutLaunch/BP_ScoutV2.ProjectileMovement` _asbp_scout_v2))
        (set `MovementComponent.Velocity` (* (`self.GetActorForwardVector` (`self.OtherPointer`)) (`KismetMathLibrary.FClamp` (`KismetMathLibrary.VSize` (`MovementComponent.Velocity` _projectilemovement)) 200.0 9999999.0)) _projectilemovement)))))

(event `self.Box.OnComponentEndOverlap`
  (params (OverlappedComponent :type "PrimitiveComponent Object Reference") (OtherActor :type "Actor Object Reference") (OtherComp :type "PrimitiveComponent Object Reference") (OtherBodyIndex :type Integer))
  (cast `/Game/MazeGame/Characters/MGHero/BP_MGHeroCharacter` OtherActor
    (:`then`
      (`self.Show Self`))
    (:`CastFailed`
      (set `self.bCanPort` true))))

(event `Show Self`
  (set `self.bCanPort` true)
  (`SceneComponent.SetVisibility` (`self.Cube1`) true false)
  (`SceneComponent.SetVisibility` (`self.Cube2`) true false)
  (`SceneComponent.SetVisibility` (`self.Cube3`) true false)
  (`SceneComponent.SetVisibility` (`self.Cube4`) true false)
  (`SceneComponent.SetVisibility` (`self.Cube5`) true false)
  (`ActorComponent.SetActive` (`self.NS_Portal`) true true))

(event `Hide Self`
  (set `self.bCanPort` false)
  (`SceneComponent.SetVisibility` (`self.Cube1`) false false)
  (`SceneComponent.SetVisibility` (`self.Cube2`) false false)
  (`SceneComponent.SetVisibility` (`self.Cube3`) false false)
  (`SceneComponent.SetVisibility` (`self.Cube4`) false false)
  (`SceneComponent.SetVisibility` (`self.Cube5`) false false)
  (`ActorComponent.Deactivate` (`self.NS_Portal`)))

(fn `SetVelocityToPrimitiveComponent`
  (params (PrimitiveComponent :type "PrimitiveComponent Object Reference"))
  (bind _returnvalue (`PrimitiveComponent.GetPhysicsLinearVelocity` PrimitiveComponent "None"))
  (`PrimitiveComponent.SetAllPhysicsLinearVelocity` PrimitiveComponent (* (`KismetMathLibrary.FClamp` (`KismetMathLibrary.VSize` _returnvalue) 200.0 9999999.0) (`self.GetActorForwardVector` (`self.OtherPointer`))) false)
  (return))

(fn `UpdateCubemapNormalVector`
  (bind _scenecapturecomponentcube (`self.SceneCaptureComponentCube`))
  (bind _scenecapturecomponentcube_2 (`/Game/MazeGame/Characters/MGHero/Abilities/PortalGun/BP_PortalMaster.SceneCaptureComponentCube` (`self.OtherPointer`)))
  (`MaterialInstanceDynamic.SetVectorParameterValue` (`self.MaterialInstDynamic`) "CustomWorldNormal" (make `LinearColor` (.x (`KismetMathLibrary.ProjectVectorOnToPlane` (`KismetMathLibrary.LessLess_VectorRotator` (`SceneComponent.GetForwardVector` _scenecapturecomponentcube_2) (`SceneComponent.K2_GetComponentRotation` _scenecapturecomponentcube_2)) (`KismetMathLibrary.LessLess_VectorRotator` (`SceneComponent.GetForwardVector` _scenecapturecomponentcube) (`SceneComponent.K2_GetComponentRotation` _scenecapturecomponentcube)))) (.y (`KismetMathLibrary.ProjectVectorOnToPlane` (`KismetMathLibrary.LessLess_VectorRotator` (`SceneComponent.GetForwardVector` _scenecapturecomponentcube_2) (`SceneComponent.K2_GetComponentRotation` _scenecapturecomponentcube_2)) (`KismetMathLibrary.LessLess_VectorRotator` (`SceneComponent.GetForwardVector` _scenecapturecomponentcube) (`SceneComponent.K2_GetComponentRotation` _scenecapturecomponentcube)))) (.z (`KismetMathLibrary.ProjectVectorOnToPlane` (`KismetMathLibrary.LessLess_VectorRotator` (`SceneComponent.GetForwardVector` _scenecapturecomponentcube_2) (`SceneComponent.K2_GetComponentRotation` _scenecapturecomponentcube_2)) (`KismetMathLibrary.LessLess_VectorRotator` (`SceneComponent.GetForwardVector` _scenecapturecomponentcube) (`SceneComponent.K2_GetComponentRotation` _scenecapturecomponentcube)))))))

(fn `UserConstructionScript`
  (bind _returnvalue (`KismetMaterialLibrary.CreateDynamicMaterialInstance` (`self.MIC`)))
  (bind _output_get (set `self.MaterialInstDynamic` _returnvalue))
  (`NiagaraComponent.SetVariableMaterial` (`self.NS_Portal`) "MIC" _output_get))