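; Gameplay ability that dashes the maze hero along the first-person camera's forward vector with Z zeroed.
; It caches hero and ASC, then reads a level-based Distance from a stats table as root-motion force strength.
; A brief constant-force task clamps exit velocity; camera shake replaces fly shake, which is re-allowed on finish.
; Forward X and Y are not renormalized, so looking up or down weakens the dash.
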(event `self.K2_ActivateAbility`
  (bind _abilityslotref (`self.AbilitySlotRef`))
  (bind (_returnvalue_x _returnvalue_y) (`KismetMathLibrary.BreakVector` (`KismetMathLibrary.Normal` (`SceneComponent.GetForwardVector` (`MGHeroCharacter.FirstPersonCamera` (`self.OwningHero`))))))
  (`self.CheckAndSetupCacheables`)
  (`UserWidget.PlayAnimation` _abilityslotref (`/Game/MazeGame/UI/Widgets/HUD/WBP_HUDAbilitySlot.ActivatingOnce` _abilityslotref) 0.0 1 "Forward" 1.0 false)
  (`self.K2_CommitAbility`)
  (bind _asbp_mghero_character (cast `/Game/MazeGame/Characters/MGHero/BP_MGHeroCharacter` (`self.OwningHero`)))
  (`/Game/MazeGame/Characters/MGHero/BP_MGHeroCharacter.StopFlyCameraShake` _asbp_mghero_character)
  (set `/Game/MazeGame/Characters/MGHero/BP_MGHeroCharacter.CanStartFlyShake` false _asbp_mghero_character)
  (`PlayerCameraManager.StartCameraShake` :`self` (`GameplayStatics.GetPlayerCameraManager` 0) :`ShakeClass` "/Game/MazeGame/Characters/MGHero/Abilities/Dash/DashShake.DashShake_C")
  (bind _asynctaskproxy (`AbilityTask_ApplyRootMotionConstantForce.ApplyRootMotionConstantForce` "None" (`KismetMathLibrary.MakeVector` _returnvalue_x _returnvalue_y) (`self.Distance`) 0.2 false null "ClampVelocity" (0.0 0.0 0.0) 600.0)
    (:`then`
      (set `self.RootMotionTask` _asynctaskproxy))
    (:`OnFinish`
      (bind _asbp_mghero_character_2 (cast `/Game/MazeGame/Characters/MGHero/BP_MGHeroCharacter` (`self.OwningHero`)))
      (set `/Game/MazeGame/Characters/MGHero/BP_MGHeroCharacter.CanStartFlyShake` true _asbp_mghero_character_2)
      (`self.K2_EndAbility`))))

(event `self.K2_OnEndAbility`
  (params (bWasCancelled :type Boolean))
  (`GameplayTask.EndTask` (`self.RootMotionTask`)))