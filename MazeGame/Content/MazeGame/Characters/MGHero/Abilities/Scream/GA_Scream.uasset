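; GA_Scream is the hero's scream gameplay ability, which breaks maze walls in the direction the first-person camera faces.
; On activation it caches the hero and ability system component, reads a level-scaled Distance from a stats table, then plays slot animation and camera shake.
; A debug-drawn multi-sphere trace along the view calls DestroyReplace on walls hit.
; It then spawns a short-lived sphere field actor at the camera and ends.
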(event `self.K2_ActivateAbility`
  (bind _abilityslotref (`self.AbilitySlotRef`))
  (bind _firstpersoncamera (`MGHeroCharacter.FirstPersonCamera` (`self.OwningHero`)))
  (bind _returnvalue (`SceneComponent.K2_GetComponentLocation` _firstpersoncamera))
  (bind _returnvalue_2 (* (`SceneComponent.GetForwardVector` _firstpersoncamera) (`self.Distance`)))
  (`self.CheckAndSetupCacheables`)
  (`UserWidget.PlayAnimation` _abilityslotref (`/Game/MazeGame/UI/Widgets/HUD/WBP_HUDAbilitySlot.ActivatingOnce` _abilityslotref) 0.0 1 "Forward" 1.0 false)
  (`self.K2_CommitAbility`)
  (`PlayerCameraManager.StartCameraShake` :`self` (`GameplayStatics.GetPlayerCameraManager` 0) :`ShakeClass` "/Game/MazeGame/Characters/MGHero/Abilities/Scream/ScreamShake.ScreamShake_C")
  (bind _outhits (`KismetSystemLibrary.SphereTraceMultiForObjects` _returnvalue (+ _returnvalue _returnvalue_2) 250.0 (`|MakeArray` "ObjectTypeQuery1" "ObjectTypeQuery2" :!type "EObjectTypeQuery Enum") false (`|MakeArray` (`GameplayStatics.GetPlayerCharacter` 0) :!type "Actor Object Reference") "ForDuration"))
  (for _array_element _outhits
    (bind _asbp_maze_wall_base (cast `/Game/MazeGame/Maze/Walls/BP_MazeWallBase` (`.HitActor` (`GameplayStatics.BreakHitResult` _array_element))))
    (`/Game/MazeGame/Maze/Walls/BP_MazeWallBase.Destroy(Replace)` _asbp_maze_wall_base 5.0))
  (bind _returnvalue_3 (`|SpawnActorFromClass` "/Game/MazeGame/Characters/MGHero/Abilities/FS_MGSphereField.FS_MGSphereField_C" (`KismetMathLibrary.MakeTransform` _returnvalue (`KismetMathLibrary.FindLookAtRotation` _returnvalue _returnvalue_2)) "Undefined" "OverrideRootScale" null null))
  (`Actor.SetLifeSpan` _returnvalue_3 0.5)
  (`self.K2_EndAbility`))