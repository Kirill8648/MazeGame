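; Gameplay ability for the maze hero that raises nearby maze walls into the air for a limited time.
; On activation it sphere-overlaps MGInstancedMeshActors around the first-person camera and swaps their instances within that radius for actors.
; Each resulting BP_MazeWallBase gets its air time, raises with no delay, then the ability ends.
; Radius and air time scale with the variable Е; a debug sphere shows the area.
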(event `self.K2_ActivateAbility`
  (bind `_е` (`self.е`))
  (bind _returnvalue (`SceneComponent.K2_GetComponentLocation` (`MGHeroCharacter.FirstPersonCamera` (`self.OwningHero`))))
  (bind _returnvalue_2 (`KismetMathLibrary.Conv_IntToDouble` (+ 3 (* `_е` 1))))
  (bind _returnvalue_3 (`KismetMathLibrary.Conv_IntToDouble` (+ 500 (* `_е` 150))))
  (`self.CheckAndSetupCacheables`)
  (`KismetSystemLibrary.DrawDebugSphere` _returnvalue _returnvalue_3 6 (struct :`R` 1.0 :`B` 0.016776 :`A` 1.0) _returnvalue_2 3.0)
  (bind _outactors (`KismetSystemLibrary.SphereOverlapActors` _returnvalue _returnvalue_3 (`|MakeArray` "ObjectTypeQuery1" "ObjectTypeQuery2" :!type "EObjectTypeQuery Enum") "/Script/MazeGame.MGInstancedMeshActor"))
  (for _array_element _outactors
    (bind _asmginstanced_mesh_actor (cast `MGInstancedMeshActor` _array_element))
    (bind _returnvalue_4 (`MGInstancedMeshActor.ReplaceInstancesWithActorsBySphereOverlap` _asmginstanced_mesh_actor _returnvalue _returnvalue_3))
    (for _array_element_2 _returnvalue_4
      (bind _asbp_maze_wall_base (cast `/Game/MazeGame/Maze/BP_MazeWallBase` _array_element_2))
      (set `/Game/MazeGame/Maze/BP_MazeWallBase.TimeInAir` _returnvalue_2 _asbp_maze_wall_base)
      (set `/Game/MazeGame/Maze/BP_MazeWallBase.DelayBeforeRaise` 0.0 _asbp_maze_wall_base)
      (`/Game/MazeGame/Maze/BP_MazeWallBase.Raise` _asbp_maze_wall_base)))
  (`self.K2_EndAbility`))

(fn `K2_CanActivateAbility`
  (params (ActorInfo :type "GameplayAbilityActorInfo Structure") (Handle :type "GameplayAbilitySpecHandle Structure"))
  (returns (RelevantTags :type "GameplayTagContainer Structure") (ReturnValue :type Boolean))
  (return (struct) true))