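; BP_ScoutV2 is the scout for the hero's ScoutLaunch ability, combining projectile movement with a scene capture camera.
; The construction script creates a dynamic instance of a custom depth fog material, stores it as ScoutCameraPP and adds it to the capture's post-process materials.
; It also copies its view distance and speed variables onto the capture and projectile movement components.
; The event graph holds only disabled placeholder events.
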(fn `UserConstructionScript`
  (bind _projectilemovement (`self.ProjectileMovement`))
  (bind _scenecapturecomponent2d (`self.SceneCaptureComponent2D`))
  (bind _returnvalue (`KismetMaterialLibrary.CreateDynamicMaterialInstance` "/Game/MazeGame/Characters/MGHero/Abilities/ScoutLaunch/PP_CustomDepthFog_Inst.PP_CustomDepthFog_Inst" "FPSCameraPP"))
  (bind _output_get (set `self.ScoutCameraPP` _returnvalue))
  (`KismetArrayLibrary.Array_Add` (`.Array` (break `WeightedBlendables` (`.WeightedBlendables` (break `PostProcessSettings` (`SceneCaptureComponent2D.PostProcessSettings` _scenecapturecomponent2d))))) (make `WeightedBlendable` 1.0 _output_get))
  (set `SceneCaptureComponent.MaxViewDistanceOverride` (`self.Max View Distance Override`) _scenecapturecomponent2d)
  (set `ProjectileMovementComponent.InitialSpeed` (`self.InitialSpeed`) _projectilemovement)
  (set `ProjectileMovementComponent.MaxSpeed` (`self.MaxSpeed`) _projectilemovement))