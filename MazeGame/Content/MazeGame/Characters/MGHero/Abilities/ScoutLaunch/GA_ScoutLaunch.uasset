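; Gameplay ability for the hero's Scout Launch, which fires a scout projectile from the first-person camera and shows its camera view overlay.
; Speed and view distance come from a stats data table by ability level, with view distance also fed to the scout's post-process material.
; A HUD hint shows the bound key, and pressing it again ends the ability.
; Ending commits cooldown and removes the scout and widgets.
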(event `self.K2_ActivateAbility`
  (bind _speed (`self.Speed`))
  (bind _abilityslotref (`self.AbilitySlotRef`))
  (bind _firstpersoncamera (`MGHeroCharacter.FirstPersonCamera` (`self.OwningHero`)))
  (`self.CheckAndSetupCacheables`)
  (`UserWidget.PlayAnimation` _abilityslotref (`/Game/MazeGame/UI/Widgets/HUD/WBP_HUDAbilitySlot.ActivatingFadeIn` _abilityslotref) 0.0 1 "Forward" 1.0 false)
  (`self.K2_CommitAbilityCost` false)
  (bind _returnvalue (`|SpawnActorFromClass` "/Game/MazeGame/Characters/MGHero/Abilities/ScoutLaunch/BP_ScoutV2.BP_ScoutV2_C" (`KismetMathLibrary.MakeTransform` (+ (`SceneComponent.K2_GetComponentLocation` _firstpersoncamera) (* (`SceneComponent.GetForwardVector` _firstpersoncamera) 100.0)) (`SceneComponent.K2_GetComponentRotation` _firstpersoncamera)) "AlwaysSpawn" "OverrideRootScale" null _speed _speed (`self.ViewDistance`) null))
  (bind _returnvalue_2 (`|CreateWidget` "/Game/MazeGame/UI/Widgets/HUD/WBP_HintText.WBP_HintText_C"))
  (bind _output_get (set `self.HintWidgetRef` _returnvalue_2))
  (`RichTextBlock.SetText` (`/Game/MazeGame/UI/Widgets/HUD/WBP_HintText.RichTextBlock` _output_get) (`KismetTextLibrary.Conv_StringToText` (`KismetStringLibrary.Concat_StrStr` "<Outlined>" (`KismetTextLibrary.Conv_TextToString` (`KismetInputLibrary.Key_GetDisplayName` (`.Key` (break `InputActionKeyMapping` (`|GetArrayItem` (`InputSettings.GetActionMappingByName` (`InputSettings.GetInputSettings`) (`KismetStringLibrary.Conv_StringToName` (`|GetEnumeratorNameAsString` (`self.AbilityInputID`))))))))) "</>" "<OutlinedLight>" (`KismetTextLibrary.Conv_TextToString` " - Return the scout") "</>")))
  (bind _returnvalue_3 (`VerticalBox.AddChildToVerticalBox` (`/Game/MazeGame/UI/Widgets/HUD/WBP_HUDProgressBars.HintsBox` (`/Game/MazeGame/UI/BP_MGHUD.ProgressBarsWidget` (`self.As BP MGHUD`))) (`self.HintWidgetRef`)))
  (`VerticalBoxSlot.SetPadding` _returnvalue_3 (make `Margin` 0.0 5.0 0.0 5.0))
  (bind _output_get_2 (set `self.ScoutProjectileV2` _returnvalue))
  (`MaterialInstanceDynamic.SetScalarParameterValue` (`/Game/MazeGame/Characters/MGHero/Abilities/ScoutLaunch/BP_ScoutV2.ScoutCameraPP` _output_get_2) "ViewDistance" (`self.ViewDistance`))
  (bind _returnvalue_4 (`|CreateWidget` "/Game/MazeGame/Characters/MGHero/Abilities/ScoutLaunch/WBP_ScoutLaunchCamera.WBP_ScoutLaunchCamera_C"))
  (bind _output_get_3 (set `self.ScoutWidgetRef` _returnvalue_4))
  (`UserWidget.AddToViewport` _output_get_3 0)
  (`AbilityTask_WaitInputPress.WaitInputPress` false
    (:`OnPress`
      (`self.K2_EndAbility`))))

(event `self.K2_OnEndAbility`
  (params (bWasCancelled :type Boolean))
  (bind _abilityslotref (`self.AbilitySlotRef`))
  (`self.K2_CommitAbilityCooldown` false)
  (`UserWidget.PlayAnimation` _abilityslotref (`/Game/MazeGame/UI/Widgets/HUD/WBP_HUDAbilitySlot.ActivatingFadeOut` _abilityslotref) 0.0 1 "Forward" 1.0 false)
  (`Widget.RemoveFromParent` (`self.ScoutWidgetRef`))
  (`Actor.K2_DestroyActor` (`self.ScoutProjectileV2`))
  (`Widget.RemoveFromParent` (`self.HintWidgetRef`)))