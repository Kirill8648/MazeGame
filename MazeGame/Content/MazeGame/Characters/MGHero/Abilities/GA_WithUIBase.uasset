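; Base gameplay ability for the maze game's hero that links abilities to the HUD.
; When added, it caches player 0's BP_MGHUD and creates an ability slot widget from its key, input ID and level, placing it in the abilities bar.
; Failed cost checks play the HUD's energy bar warning animation, and failed cooldown checks play the slot's cooldown warning, using those cached references.
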(event `self.K2_OnAbilityAdded`
  (bind _asbp_mghud (cast `/Game/MazeGame/UI/BP_MGHUD` (`PlayerController.GetHUD` (`GameplayStatics.GetPlayerController` 0)))
    (:`then`
      (set `self.As BP MGHUD` _asbp_mghud)
      (bind _returnvalue (`|CreateWidget` "/Game/MazeGame/UI/Widgets/HUD/WBP_HUDAbilitySlot.WBP_HUDAbilitySlot_C" null (`self.AbilityKey`) (`self.AbilityInputID`) (`self.GetAbilityLevel`)))
      (set `self.AbilitySlotRef` _returnvalue)
      (bind _progressbarswidget (`/Game/MazeGame/UI/BP_MGHUD.ProgressBarsWidget` (`self.As BP MGHUD`))
        (:`then`
          (bind _returnvalue_2 (`HorizontalBox.AddChildToHorizontalBox` (`/Game/MazeGame/UI/Widgets/HUD/WBP_HUDProgressBars.Abilities` _progressbarswidget) (`self.AbilitySlotRef`)))
          (`HorizontalBoxSlot.SetPadding` _returnvalue_2 (make `Margin` 2.5 0.0 2.5)))
        (:`else`)))
    (:`CastFailed`
      (`KismetSystemLibrary.PrintString` "Cast to BP_MGHUD failed in GA_WithUIBase" true true (struct :`R` 1.0 :`A` 1.0) 10.0))))

(fn `K2_OnAbilityCheckCooldown`
  (params (ReturnValue :type Boolean))
  (if (not ReturnValue)
    (bind _abilityslotref (`self.AbilitySlotRef`)
      (:`then`
        (`UserWidget.PlayAnimation` _abilityslotref (`/Game/MazeGame/UI/Widgets/HUD/WBP_HUDAbilitySlot.CooldownWarning` _abilityslotref) 0.0 1 "Forward" 1.0 false))
      (:`else`
        (`KismetSystemLibrary.PrintString` "AbilitySlotRef is not valid in K2_OnAbilityCheckCooldown in GA_WithUIBase" true true (struct :`R` 1.0 :`B` 1.0 :`A` 1.0) 20.0)))))

(fn `K2_OnAbilityCheckCost`
  (params (ReturnValue :type Boolean))
  (if (not ReturnValue)
    (bind _as_bp_mghud (`self.As BP MGHUD`)
      (:`then`
        (bind _progressbarswidget (`/Game/MazeGame/UI/BP_MGHUD.ProgressBarsWidget` _as_bp_mghud))
        (`UserWidget.PlayAnimation` _progressbarswidget (`/Game/MazeGame/UI/Widgets/HUD/WBP_HUDProgressBars.EnergyBarWarning` _progressbarswidget) 0.0 1 "Forward" 1.0 false))
      (:`else`
        (`KismetSystemLibrary.PrintString` "As BP_MGHUD is not valid in K2_OnAbilityCheckCost in GA_WithUIBase" true true (struct :`R` 1.0 :`B` 1.0 :`A` 1.0) 20.0)))))