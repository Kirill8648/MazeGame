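; First-person hero character Blueprint for the maze game, handling camera feedback, fall damage, the pause menu, death screen and HUD ability-slot removal.
; Movement events drive jump, landing, walk and airborne camera shakes, with looping timers repeating walk and flight shakes and speed exponentially scaling landing and air shakes.
; Landing applies a SetByCaller gameplay effect based on vertical speed and max health.
; BeginPlay adds a custom-depth post-process material; debug keys trigger death and launch.
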(event `self.K2_RemoveAbilitySlotFromHUD`
  (params (SlotID :type "EMGAbilityInputID Enum (by ref)" :default "None"))
  ;[1 0.8196 0.3765] HUD
  (bind _asbp_mghud (cast `/Game/MazeGame/UI/BP_MGHUD` (`PlayerController.GetHUD` (`GameplayStatics.GetPlayerController` 0)))
    (:`then`
      (`/Game/MazeGame/UI/BP_MGHUD.RemoveAbilitySlot` _asbp_mghud SlotID))
    (:`CastFailed`
      (`KismetSystemLibrary.PrintString` "cast to hud in character failed"))))

(event `InputAction|Open/ClosePauseMenu`
  (params (Key :type "Key Structure"))
  (bind _returnvalue (`GameplayStatics.GetPlayerController` 0))
  (bind _pausemenuref (`self.PauseMenuRef`))
  (bind (_x _y) (`KismetMathLibrary.BreakVector2D` (`WidgetLayoutLibrary.GetViewportSize`)))
  ;[1 0.8196 0.3765] Menu
  (:`Pressed`
    (bind _returnvalue_2 (`|CreateWidget` "/Game/MazeGame/UI/Widgets/WBP_PauseMenu.WBP_PauseMenu_C"))
    (set `self.PauseMenuRef` _returnvalue_2)
    (set `PlayerController.bShowMouseCursor` true _returnvalue)
    (`WidgetBlueprintLibrary.SetInputMode_UIOnlyEx` _returnvalue _pausemenuref)
    (`UserWidget.AddToViewport` _pausemenuref 0)
    (`Widget.SetKeyboardFocus` _pausemenuref)
    (`GameplayStatics.SetGamePaused` true)
    (`PlayerController.SetMouseLocation` _returnvalue (`KismetMathLibrary.FTrunc` (/ _x 2.0)) (`KismetMathLibrary.FTrunc` (/ _y 2.0)))))

(event `InputAction|Jump`
  (params (Key :type "Key Structure"))
  (bind _returnvalue (`KismetMathLibrary.RandomBool`))
  (bind _returnvalue_2 (`GameplayStatics.GetPlayerCameraManager` 0))
  ;[0.1945 1 0.2943] Camera Shakes
  (:`Pressed`
    (`self.Jump`)
    (if (not (`NavMovementComponent.IsFalling` (`self.CharacterMovement`)))
      (`PlayerCameraManager.StopCameraShake` _returnvalue_2 (`self.LandCSRef`) false)
      (`MatineeCameraShake.StartMatineeCameraShakeFromSource` _returnvalue_2 (select `bool` (`GameplayTagAssetInterface.HasMatchingGameplayTag` (`AbilitySystemBlueprintLibrary.GetAbilitySystemComponent` self) (struct :`TagName` "State.Sprinting")) :`false` (select `bool` _returnvalue :`false` "/Game/MazeGame/Characters/MGHero/ChameraShakes/JumpMatineeCameraShakeA.JumpMatineeCameraShakeA_C" :`true` "/Game/MazeGame/Characters/MGHero/ChameraShakes/JumpMatineeCameraShakeB.JumpMatineeCameraShakeB_C" :!type "MatineeCameraShake Class Reference") :`true` (select `bool` _returnvalue :`false` "/Game/MazeGame/Characters/MGHero/ChameraShakes/JumpSprintMatineeCSA.JumpSprintMatineeCSA_C" :`true` "/Game/MazeGame/Characters/MGHero/ChameraShakes/JumpSprintMatineeCSB.JumpSprintMatineeCSB_C" :!type "MatineeCameraShake Class Reference"))))))

(event `self.OnLanded`
  (params (Hit :type "HitResult Structure (by ref)"))
  (bind (_returnvalue_x _returnvalue_y _returnvalue_z) (`KismetMathLibrary.BreakVector` (`self.GetVelocity`)))
  (bind _returnvalue (`GameplayStatics.GetPlayerCameraManager` 0))
  (bind _returnvalue_2 (`AbilitySystemBlueprintLibrary.GetAbilitySystemComponent` self))
  (bind _returnvalue_3 (`KismetMathLibrary.FClamp` (`KismetMathLibrary.Exp` (/ (`KismetMathLibrary.VSize` (`self.GetVelocity`)) 700.0)) 0.0 50.0))
  (bind _returnvalue_4 (`AbilitySystemBlueprintLibrary.AssignTagSetByCallerMagnitude` (`AbilitySystemComponent.MakeOutgoingSpec` :`self` _returnvalue_2 :`GameplayEffectClass` "/Game/MazeGame/Characters/MGHero/GamepalyEffects/GE_LandDamage.GE_LandDamage_C" :`Level` 1.0) (struct :`TagName` "SetByCaller.FallDamage") (`KismetMathLibrary.Conv_IntToDouble` (`KismetMathLibrary.Round` (* (`KismetMathLibrary.FClamp` (`KismetMathLibrary.NormalizeToRange` (`KismetMathLibrary.Abs` _returnvalue_z) 1200.0 1900.0)) (`self.GetMaxHealth`) -1.0)))))
  ;[0.1945 1 0.2943] Camera Shakes
  (`AbilitySystemComponent.BP_ApplyGameplayEffectSpecToSelf` _returnvalue_2 _returnvalue_4)
  (bind _returnvalue_5 (`MatineeCameraShake.StartMatineeCameraShakeFromSource` _returnvalue "/Game/MazeGame/Characters/MGHero/ChameraShakes/LandMatineeCameraShake.LandMatineeCameraShake_C" null _returnvalue_3))
  (`MatineeCameraShake.StartMatineeCameraShakeFromSource` _returnvalue "/Game/MazeGame/Characters/MGHero/ChameraShakes/LandNoiseShake.LandNoiseShake_C" null _returnvalue_3)
  (set `self.LandCSRef` _returnvalue_5)
  (`self.StopFlyCameraShake`))

(event `self.StartWalkCameraShake`
  (params (DoShakeOnStart :type "Integer (by ref)"))
  ;[0.1945 1 0.2943] Camera Shakes
  (if (`KismetMathLibrary.Conv_IntToBool` DoShakeOnStart)
    (bind _returnvalue (`MatineeCameraShake.StartMatineeCameraShakeFromSource` (`GameplayStatics.GetPlayerCameraManager` 0) (`self.WalkCameraShakeClass`)))
    (set `self.WalkCameraShakeRef` _returnvalue))
  (bind _returnvalue_2 (`KismetSystemLibrary.K2_SetTimerDelegate` (delegate `ApplyWalkCameraShake`) (`self.WalkAnimLength`) true))
  (set `self.CameraShaketimerHandle` _returnvalue_2))

(event `ApplyWalkCameraShake`
  ;[0.1945 1 0.2943] Camera Shakes
  (bind _returnvalue (`MatineeCameraShake.StartMatineeCameraShakeFromSource` (`GameplayStatics.GetPlayerCameraManager` 0) (`self.WalkCameraShakeClass`)))
  (set `self.WalkCameraShakeRef` _returnvalue))

(event `self.StopWalkCameraShake`
  (params (Immediately :type "Integer (by ref)") (ClearHandle :type "Integer (by ref)"))
  ;[0.1945 1 0.2943] Camera Shakes
  (if (`KismetMathLibrary.Conv_IntToBool` ClearHandle)
    (`KismetSystemLibrary.K2_ClearAndInvalidateTimerHandle` (`self.CameraShaketimerHandle`)))
  (`PlayerCameraManager.StopCameraShake` (`GameplayStatics.GetPlayerCameraManager` 0) (`self.WalkCameraShakeRef`) (`KismetMathLibrary.Conv_IntToBool` Immediately)))

(event `self.K2_OnMovementModeChanged`
  (params (PrevMovementMode :type "EMovementMode Enum" :default "MOVE_None") (NewMovementMode :type "EMovementMode Enum" :default "MOVE_None") (PrevCustomMode :type Byte) (NewCustomMode :type Byte))
  ;[1 1 1] Camera Shake In Air
  (if (`|EnumEquality` PrevMovementMode "MOVE_Flying")
    (`KismetSystemLibrary.Delay` 0.0)
    (if (`GameplayTagAssetInterface.HasMatchingGameplayTag` (`AbilitySystemBlueprintLibrary.GetAbilitySystemComponent` self) (struct :`TagName` "State.Dead")) :!label _label
      (`self.StopWalkCameraShake` 1 1)
      (`self.StopFlyCameraShake`)
      (elif (`self.CanStartFlyShake`)
        (bind _returnvalue (`MatineeCameraShake.StartMatineeCameraShakeFromSource` (`GameplayStatics.GetPlayerCameraManager` 0) "/Game/MazeGame/Characters/MGHero/ChameraShakes/FlyingCS.FlyingCS_C" null (- (`KismetMathLibrary.Exp` (/ (`KismetMathLibrary.VSize` (`self.GetVelocity`)) 1000.0)) 1.0)))
        (set `self.FlyCameraShakeRef` _returnvalue)
        (bind _returnvalue_2 (`KismetSystemLibrary.K2_SetTimerDelegate` (delegate `ApplyFlyShake`) (`self.FlyShakeLength`) true))
        (set `self.FlyShakeTimerHandle` _returnvalue_2)))))

(event `self.OnJumped`
  ;[1 1 1] Camera Shake In Air
  (goto _label))

(event `self.OnLaunched`
  (params (LaunchVelocity :type "Vector Structure") (bXYOverride :type Boolean) (bZOverride :type Boolean))
  ;[1 1 1] Camera Shake In Air
  (`KismetSystemLibrary.Delay` 0.0)
  (goto _label))

(event `self.OnWalkingOffLedge`
  (params (PreviousFloorImpactNormal :type "Vector Structure (by ref)") (PreviousFloorContactNormal :type "Vector Structure (by ref)") (PreviousLocation :type "Vector Structure (by ref)") (TimeDelta :type "Float (single-precision)"))
  ;[1 1 1] Camera Shake In Air
  (goto _label))

(event `ApplyFlyShake`
  ;[1 1 1] Camera Shake In Air
  (bind _returnvalue (`MatineeCameraShake.StartMatineeCameraShakeFromSource` (`GameplayStatics.GetPlayerCameraManager` 0) "/Game/MazeGame/Characters/MGHero/ChameraShakes/FlyingCS.FlyingCS_C" null (- (`KismetMathLibrary.Exp` (/ (`KismetMathLibrary.VSize` (`self.GetVelocity`)) 1000.0)) 1.0)))
  (set `self.FlyCameraShakeRef` _returnvalue))

(event `StopFlyCameraShake`
  ;[1 1 1] Camera Shake In Air
  (`KismetSystemLibrary.K2_ClearAndInvalidateTimerHandle` (`self.FlyShakeTimerHandle`))
  (`PlayerCameraManager.StopCameraShake` (`GameplayStatics.GetPlayerCameraManager` 0) (`self.FlyCameraShakeRef`) false))

(event `self.K2_OnDied`
  (bind _returnvalue (`GameplayStatics.GetPlayerController` 0))
  (bind (_x _y) (`KismetMathLibrary.BreakVector2D` (`WidgetLayoutLibrary.GetViewportSize`)))
  ;[1 0 0] Death
  (`KismetSystemLibrary.Delay` 3.0)
  (bind _returnvalue_2 (`|CreateWidget` "/Game/MazeGame/UI/Widgets/WBP_DiedScreen.WBP_DiedScreen_C"))
  (`UserWidget.AddToViewport` _returnvalue_2 0)
  (bind _completestatscombined (`/Game/MazeGame/UI/Widgets/WBP_LevelFinishedScreen.CompleteStatsCombined` _returnvalue_2))
  (`UserWidget.PlayAnimation` _returnvalue_2 _completestatscombined 0.0 1 "Forward" 1.0 false)
  (`WidgetBlueprintLibrary.SetInputMode_UIOnlyEx` _returnvalue null)
  (`PlayerController.SetMouseLocation` _returnvalue (`KismetMathLibrary.FTrunc` (/ _x 2.0)) (`KismetMathLibrary.FTrunc` (/ _y 2.0)))
  (`KismetSystemLibrary.Delay` (`WidgetAnimation.GetEndTime` _completestatscombined))
  (set `PlayerController.bShowMouseCursor` true _returnvalue))

(event `Key|B`
  (params (Key :type "Key Structure"))
  ;[1 0 0.956] Debug
  (:`Pressed`
    (`self.Die`)
    (`self.StopFlyCameraShake`)
    (`self.StopWalkCameraShake` 1 1)))

(event `Key|L`
  (params (Key :type "Key Structure"))
  ;[1 0 0.956] Debug
  (:`Pressed`
    (`self.LaunchCharacter` (0.0 0.0 5000.0))))

(event `self.ReceiveBeginPlay`
  (bind _returnvalue (`KismetMaterialLibrary.CreateDynamicMaterialInstance` "/Game/MazeGame/Characters/MGHero/PP_CustomDepth_Inst.PP_CustomDepth_Inst" "FPSCameraPP"))
  (bind _output_get (set `self.FPSCameraPP` _returnvalue))
  (`KismetArrayLibrary.Array_Add` (`.Array` (break `WeightedBlendables` (`.WeightedBlendables` (break `PostProcessSettings` (`CameraComponent.PostProcessSettings` (`self.FirstPersonCamera`)))))) (make `WeightedBlendable` 1.0 _output_get)))

(fn `UserConstructionScript`)