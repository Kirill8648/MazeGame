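; Maze floor trap that costs the hero a small number of coins when stepped on.
; On hero overlap with the trap box, DoTrap applies the GE_Minus5Coins gameplay effect through the hero's Ability System Component.
; It then spawns a tinted Niagara burst above the cube and destroys the cube and collision box, so it fires only once.
; The construction script applies the trap material to the cube.
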(event `self.TrapBoxCollision.OnComponentBeginOverlap`
  (params (OverlappedComponent :type "PrimitiveComponent Object Reference") (OtherActor :type "Actor Object Reference") (OtherComp :type "PrimitiveComponent Object Reference") (OtherBodyIndex :type Integer) (bFromSweep :type Boolean) (SweepResult :type "HitResult Structure (by ref)"))
  (bind _asbp_mghero_character (cast `/Game/MazeGame/Characters/MGHero/BP_MGHeroCharacter` OtherActor))
  (`self.DoTrap` _asbp_mghero_character)
  (bind _returnvalue (`NiagaraFunctionLibrary.SpawnSystemAtLocation` "/Game/MazeGame/Maze/Floor/NS_Trap.NS_Trap" (+ (`SceneComponent.K2_GetComponentLocation` (`self.Cube`)) (0.0 0.0 100.0))))
  (`NiagaraComponent.SetVariableLinearColor` _returnvalue "MainColor" (`self.Color`))
  (`ActorComponent.K2_DestroyComponent` (`self.Cube`))
  (`ActorComponent.K2_DestroyComponent` (`self.TrapBoxCollision`)))

(fn `DoTrap`
  (params (Hero :type "/Game/MazeGame/Characters/MGHero/BP_MGHeroCharacter Object Reference"))
  (`AbilitySystemComponent.BP_ApplyGameplayEffectToSelf` :`self` (`AbilitySystemBlueprintLibrary.GetAbilitySystemComponent` Hero) :`GameplayEffectClass` "/Game/MazeGame/Maze/CellObjects/GE_Minus5Coins.GE_Minus5Coins_C"))

(fn `UserConstructionScript`
  (`PrimitiveComponent.SetMaterial` (`self.Cube`) 0 (`self.TrapMat`)))