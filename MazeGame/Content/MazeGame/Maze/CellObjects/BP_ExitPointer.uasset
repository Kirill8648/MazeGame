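; Maze exit pointer pad that turns an arrow roughly toward the level exit while the hero stands on it.
; On overlap, a hero with low energy only triggers the HUD energy warning; otherwise it receives a gameplay effect.
; The arrow then eases toward the first exit volume, skewed by a random yaw fixed at BeginPlay, as the cube sinks and shows a disabled material.
; Leaving restores the cached poses and material.
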(event `self.ReceiveBeginPlay`
  (set `self.RandomizedAngle` (`KismetMathLibrary.RandomFloatInRange` -100.0 100.0))
  (set `self.ArrowCache` (`SceneComponent.K2_GetComponentRotation` (`self.Arrow`)))
  (set `self.CubePosCache` (`SceneComponent.RelativeLocation` (`self.Cube`))))

(event `self.Box.OnComponentBeginOverlap`
  (params (OverlappedComponent :type "PrimitiveComponent Object Reference") (OtherActor :type "Actor Object Reference") (OtherComp :type "PrimitiveComponent Object Reference") (OtherBodyIndex :type Integer) (bFromSweep :type Boolean) (SweepResult :type "HitResult Structure (by ref)"))
  (bind _cube (`self.Cube`))
  (bind _asbp_mghero_character (cast `/Game/MazeGame/Characters/MGHero/BP_MGHeroCharacter` OtherActor))
  (if (`self.CheckConsumable` _asbp_mghero_character)
    (`self.PlayAnim`)
    (else
      (`AbilitySystemComponent.BP_ApplyGameplayEffectToSelf` :`self` (`AbilitySystemBlueprintLibrary.GetAbilitySystemComponent` _asbp_mghero_character) :`GameplayEffectClass` (`self.EffectToApply`))
      (bind _outactors (`GameplayStatics.GetAllActorsOfClass` "/Game/MazeGame/Maze/BP_ExitlevelVolume.BP_ExitlevelVolume_C"))
      (`|ExecutionSequence`
        (:`then_0`
          (`KismetSystemLibrary.MoveComponentTo` (`self.Arrow`) (0.0 0.0 0.0) (`KismetMathLibrary.ComposeRotators` (`KismetMathLibrary.FindLookAtRotation` (`self.K2_GetActorLocation`) (`self.K2_GetActorLocation` (`|GetArrayItem` _outactors))) (`KismetMathLibrary.MakeRotator` 0.0 0.0 (`self.RandomizedAngle`))) true true 0.5 true))
        (:`then_1`
          (`KismetSystemLibrary.MoveComponentTo` _cube (0.0 0.0 -145.0) (struct) true true 0.3)
          (`PrimitiveComponent.SetMaterial` _cube 0 (`self.MaterialDisabled`)))))))

(event `self.Box.OnComponentEndOverlap`
  (params (OverlappedComponent :type "PrimitiveComponent Object Reference") (OtherActor :type "Actor Object Reference") (OtherComp :type "PrimitiveComponent Object Reference") (OtherBodyIndex :type Integer))
  (bind _cube (`self.Cube`))
  (cast `/Game/MazeGame/Characters/MGHero/BP_MGHeroCharacter` OtherActor)
  (`|ExecutionSequence`
    (:`then_0`
      (`KismetSystemLibrary.MoveComponentTo` (`self.Arrow`) (0.0 0.0 0.0) (`self.ArrowCache`) false false 0.3 true))
    (:`then_2`
      (`KismetSystemLibrary.MoveComponentTo` _cube (`self.CubePosCache`) (struct) true true 0.3)
      (`PrimitiveComponent.SetMaterial` _cube 0 (`self.Material`)))))

(fn `CheckConsumable`
  (params (Character :type "/Game/MazeGame/Characters/MGHero/BP_MGHeroCharacter Object Reference"))
  (returns (CantActivate :type Boolean))
  (return (< (`MGCharacterBase.GetEnergy` Character) 20.0)))

(fn `PlayAnim`
  (bind _asbp_mghud (cast `/Game/MazeGame/UI/BP_MGHUD` (`PlayerController.GetHUD` (`GameplayStatics.GetPlayerController` 0))))
  (bind _progressbarswidget (`/Game/MazeGame/UI/BP_MGHUD.ProgressBarsWidget` _asbp_mghud))
  (`UserWidget.PlayAnimation` _progressbarswidget (`/Game/MazeGame/UI/Widgets/HUD/WBP_HUDProgressBars.EnergyBarWarning` _progressbarswidget) 0.0 1 "Forward" 1.0 false))

(fn `UserConstructionScript`)