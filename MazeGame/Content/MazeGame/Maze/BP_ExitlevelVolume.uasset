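; BP_ExitlevelVolume is a maze-game trigger volume that ends the level when the hero character overlaps its box.
; It adds the hero's coins to the current save object's total in memory and clears the game mode's timer.
; It then shows an animated level-finished widget, switches to UI-only input and centers the mouse.
; Parallel delays reveal the cursor when the animation ends and stop the hero's movement after a short pause.
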(event `self.Box.OnComponentBeginOverlap`
  (params (OverlappedComponent :type "PrimitiveComponent Object Reference") (OtherActor :type "Actor Object Reference") (OtherComp :type "PrimitiveComponent Object Reference") (OtherBodyIndex :type Integer) (bFromSweep :type Boolean) (SweepResult :type "HitResult Structure (by ref)"))
  (bind _returnvalue (`GameplayStatics.GetPlayerController` 0))
  (bind (_x _y) (`KismetMathLibrary.BreakVector2D` (`WidgetLayoutLibrary.GetViewportSize`)))
  (bind _charactermovement (`Character.CharacterMovement` (`self.As BP MGHero Character`)))
  (bind _playercurrentcoinsnumber (`MGSaveGame.PlayerCurrentCoinsNumber` (`MGPlayerDataSubsystem.CurrentlyLoadedSaveGameObject` (subsystem `MGPlayerDataSubsystem`))))
  (bind _asbp_mghero_character (cast `/Game/MazeGame/Characters/MGHero/BP_MGHeroCharacter` OtherActor))
  (set `self.As BP MGHero Character` _asbp_mghero_character)
  (`KismetSystemLibrary.PrintString` "LEVEL FINISHED" true true (struct :`G` 1.0 :`A` 1.0) 10.0)
  (`|VariableSetRef` _playercurrentcoinsnumber (`KismetMathLibrary.FTrunc` (+ (`MGCharacterBase.GetCoins` (`self.As BP MGHero Character`)) _playercurrentcoinsnumber)))
  (bind _asbp_maze_generation_game_mode (cast `/Game/MazeGame/Core/BP_MazeGenerationGameMode` (`GameplayStatics.GetGameMode`)))
  (`/Game/MazeGame/Core/BP_MazeGenerationGameMode.ClearTimer` _asbp_maze_generation_game_mode)
  (bind _returnvalue_2 (`|CreateWidget` "/Game/MazeGame/UI/Widgets/WBP_LevelFinishedScreen.WBP_LevelFinishedScreen_C"))
  (`UserWidget.AddToViewport` _returnvalue_2 0)
  (bind _completestatscombined (`/Game/MazeGame/UI/Widgets/WBP_LevelFinishedScreen.CompleteStatsCombined` _returnvalue_2))
  (`UserWidget.PlayAnimation` _returnvalue_2 _completestatscombined 0.0 1 "Forward" 1.0 false)
  (`WidgetBlueprintLibrary.SetInputMode_UIOnlyEx` _returnvalue null)
  (`PlayerController.SetMouseLocation` _returnvalue (`KismetMathLibrary.FTrunc` (/ _x 2.0)) (`KismetMathLibrary.FTrunc` (/ _y 2.0)))
  (`|ExecutionSequence`
    (:`then_0`
      (`KismetSystemLibrary.Delay` (`WidgetAnimation.GetEndTime` _completestatscombined))
      (set `PlayerController.bShowMouseCursor` true _returnvalue))
    (:`then_1`
      (`KismetSystemLibrary.Delay` 2.0)
      (`CharacterMovementComponent.DisableMovement` _charactermovement)
      (set `MovementComponent.Velocity` (0.0 0.0 0.0) _charactermovement))))

(fn `UserConstructionScript`)