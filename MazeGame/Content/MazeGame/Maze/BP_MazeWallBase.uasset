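; Base maze wall Blueprint whose simple mesh can temporarily lift 500 units and then drop back.
; Raise sets an in-air guard, caches the mesh's relative location, waits a configurable delay, then eases the mesh up with MoveComponentTo.
; After a time in the air it calls Return, which moves the mesh back to the cached location and clears the guard.
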(event `Raise`
  (bind _wallsimplemesh (`self.WallSimpleMesh`))
  (bind _relativelocation (`SceneComponent.RelativeLocation` _wallsimplemesh))
  (if (not (`self.bUpInAir`))
    (set `self.bUpInAir` (not (`self.bUpInAir`)))
    (set `self.MeshRelLocCache` _relativelocation)
    (`KismetSystemLibrary.Delay` (`self.DelayBeforeRaise`))
    (`KismetSystemLibrary.MoveComponentTo` _wallsimplemesh (+ _relativelocation (0.0 0.0 500.0)) (`SceneComponent.RelativeRotation` _wallsimplemesh) true true 1.0)
    (`KismetSystemLibrary.Delay` (`self.TimeInAir`))
    (`self.Return`)))

(event `Return`
  (bind _wallsimplemesh (`self.WallSimpleMesh`))
  (if (`self.bUpInAir`)
    (`KismetSystemLibrary.MoveComponentTo` _wallsimplemesh (`self.MeshRelLocCache`) (`SceneComponent.RelativeRotation` _wallsimplemesh) false true 1.0)
    (set `self.bUpInAir` (not (`self.bUpInAir`)))))

(fn `UserConstructionScript`)