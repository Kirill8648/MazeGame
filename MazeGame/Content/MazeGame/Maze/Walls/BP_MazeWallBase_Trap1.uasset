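; Trap variant of a maze wall that jumps at the hero and slams down when they overlap its TrapCatch volume.
; The wall mesh moves high above the hero's position in its cached starting space, then quickly drops lower.
; A debug-drawn box trace then hits pawns, applying SetByCaller damage through GAS and launching characters horizontally away.
; Afterward the mesh moves back to the relative location cached at BeginPlay.
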(event `self.ReceiveBeginPlay`
  (set `self.TrapRelPosCache` (`SceneComponent.RelativeLocation` (`self.WallSimpleMesh`)))
  (set `self.WorldTransformCache` (`SceneComponent.K2_GetComponentToWorld` (`self.WallSimpleMesh`))))

(event `self.TrapCatch.OnComponentBeginOverlap`
  (params (OverlappedComponent :type "PrimitiveComponent Object Reference") (OtherActor :type "Actor Object Reference") (OtherComp :type "PrimitiveComponent Object Reference") (OtherBodyIndex :type Integer) (bFromSweep :type Boolean) (SweepResult :type "HitResult Structure (by ref)"))
  (bind _wallsimplemesh (`self.WallSimpleMesh`))
  (bind _wallsimplemesh_2 (`self.WallSimpleMesh`))
  (bind _returnvalue (`SceneComponent.K2_GetComponentLocation` _wallsimplemesh))
  (bind _asbp_mghero_character (cast `/Game/MazeGame/Characters/MGHero/BP_MGHeroCharacter` OtherActor))
  (bind _returnvalue_2 (`KismetMathLibrary.InverseTransformLocation` (`self.WorldTransformCache`) (`SceneComponent.K2_GetComponentLocation` (`Character.CapsuleComponent` _asbp_mghero_character))))
  (`KismetSystemLibrary.MoveComponentTo` _wallsimplemesh_2 (+ _returnvalue_2 (0.0 0.0 500.0)) (struct) false false 0.1)
  (`KismetSystemLibrary.MoveComponentTo` _wallsimplemesh_2 (+ _returnvalue_2 (0.0 0.0 200.0)) (struct) false false 0.1)
  (bind _outhits (`KismetSystemLibrary.BoxTraceMultiForObjects` :`Start` _returnvalue :`End` _returnvalue :`HalfSize` (250.0 28.0 500.0) :`Orientation` (`SceneComponent.K2_GetComponentRotation` _wallsimplemesh) :`ObjectTypes` (`|MakeArray` "ObjectTypeQuery3" :!type "EObjectTypeQuery Enum") :`DrawDebugType` "ForDuration"))
  (for _array_element _outhits
    (bind (_bblockinghit _binitialoverlap _time _distance _location _impactpoint _normal _impactnormal _physmat _hitactor) (`GameplayStatics.BreakHitResult` _array_element))
    (bind _returnvalue_3 (`AbilitySystemBlueprintLibrary.GetAbilitySystemComponent` _hitactor))
    (bind _returnvalue_4 (`AbilitySystemBlueprintLibrary.AssignTagSetByCallerMagnitude` (`AbilitySystemComponent.MakeOutgoingSpec` :`self` _returnvalue_3 :`GameplayEffectClass` "/Game/MazeGame/Characters/MGHero/GamepalyEffects/GE_InstantDamageSetByCaller.GE_InstantDamageSetByCaller_C" :`Level` 1.0) (struct :`TagName` "SetByCaller.Damage") -20.0))
    (`AbilitySystemComponent.BP_ApplyGameplayEffectSpecToSelf` _returnvalue_3 _returnvalue_4)
    (bind _ascharacter (cast `Character` _hitactor))
    (`Character.LaunchCharacter` _ascharacter (* (`KismetMathLibrary.MakeVector` (.x (`KismetMathLibrary.GetDirectionUnitVector` (`SceneComponent.K2_GetComponentLocation` (`self.WallSimpleMesh`)) (`self.K2_GetActorLocation` _hitactor))) (.y (`KismetMathLibrary.GetDirectionUnitVector` (`SceneComponent.K2_GetComponentLocation` (`self.WallSimpleMesh`)) (`self.K2_GetActorLocation` _hitactor)))) 2000.0) false false))
  (`KismetSystemLibrary.MoveComponentTo` _wallsimplemesh_2 (`self.TrapRelPosCache`) (struct) false false 0.15))

(fn `UserConstructionScript`
  (`parent.UserConstructionScript`))