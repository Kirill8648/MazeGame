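; Base maze wall that can rise into the air and slam back down, hurting and knocking away characters beneath it.
; Raise waits a delay, eases the mesh upward, then starts a timer that calls Return, which can also cut the cycle short.
; Return drops the wall quickly; landing triggers a camera shake, then applies a GAS damage effect and outward launch to characters in LandDamageTrigger.
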(event `Raise`
  (set `self.bUpInAir` (not (`self.bUpInAir`)))
  (bind _returnvalue (`KismetSystemLibrary.K2_SetTimerDelegate` (delegate `ActuallyRaise`) (`self.DelayBeforeRaise`)))
  (set `self.DelayBeforeRaiseHandle` _returnvalue))

(event `ActuallyRaise`
  (bind _wallsimplemesh (`self.WallSimpleMesh`))
  (bind _relativerotation (`SceneComponent.RelativeRotation` _wallsimplemesh))
  (`|ExecutionSequence`
    (:`then_0`
      (`KismetSystemLibrary.MoveComponentTo` _wallsimplemesh (+ (`self.RelLocStart`) (0.0 0.0 500.0)) _relativerotation true true 1.0 :!label _label)
      (bind _returnvalue (`KismetSystemLibrary.K2_SetTimerDelegate` (delegate `Return`) (`self.TimeInAir`)))
      (set `self.TimeInAirHandle` _returnvalue))
    (:`then_1`
      (goto _label_2 :!via `Stop`))))

(event `Return`
  (if (`self.bUpInAir`)
    (`KismetSystemLibrary.K2_ClearAndInvalidateTimerHandle` (`self.TimeInAirHandle`))
    (`KismetSystemLibrary.K2_ClearAndInvalidateTimerHandle` (`self.DelayBeforeRaiseHandle`))
    (`|ExecutionSequence`
      (:`then_0`
        (goto _label :!via `Stop`))
      (:`then_1`
        (`KismetSystemLibrary.MoveComponentTo` (`self.WallSimpleMesh`) (`self.RelLocStart`) (`SceneComponent.RelativeRotation` (`self.WallSimpleMesh`)) false true 0.1 :!label _label_2)
        (set `self.bUpInAir` (not (`self.bUpInAir`)))
        (`GameplayStatics.PlayWorldCameraShake` "/Game/MazeGame/Characters/MGHero/Abilities/RaiseWalls/WallLandCameraShake.WallLandCameraShake_C" (`SceneComponent.K2_GetComponentLocation` (`self.LandDamageTrigger`)) 0.0 1000.0 0.1)
        (for _array_element (`PrimitiveComponent.GetOverlappingActors` (`self.LandDamageTrigger`) "/Script/MazeGame.MGCharacterBase")
          (`AbilitySystemComponent.BP_ApplyGameplayEffectToSelf` :`self` (`AbilitySystemBlueprintLibrary.GetAbilitySystemComponent` _array_element) :`GameplayEffectClass` "/Game/MazeGame/Characters/MGHero/Abilities/RaiseWalls/GE_WallLandDamage.GE_WallLandDamage_C" :`Level` 0.0)
          (bind _ascharacter (cast `Character` _array_element))
          (`Character.LaunchCharacter` _ascharacter (* (`KismetMathLibrary.GetDirectionUnitVector` (`SceneComponent.K2_GetComponentLocation` (`self.LandDamageTrigger`)) (`self.K2_GetActorLocation` _array_element)) 1000.0) false false))))))

(fn `UserConstructionScript`
  (set `self.RelLocStart` (`SceneComponent.RelativeLocation` (`self.WallSimpleMesh`))))