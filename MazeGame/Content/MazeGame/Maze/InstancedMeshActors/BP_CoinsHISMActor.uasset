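; Coin field actor for the maze game that renders a large grid of coins as instances of one hierarchical instanced mesh.
; On BeginPlay, nested loops add evenly spaced instances in local space.
; When a BP_MGHeroCharacter overlaps the component, a small sphere query at the sweep impact point finds the touched instance and removes it.
; No score or pickup reward is handled here.
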(event `self.ReceiveBeginPlay`
  (for _index (range 101)
    (for _index_2 (range 101)
      (`InstancedStaticMeshComponent.AddInstance` (`self.HierarchicalInstancedMesh`) (`KismetMathLibrary.MakeTransform` (`KismetMathLibrary.MakeVector` (`KismetMathLibrary.Conv_IntToDouble` (* _index 1000)) (`KismetMathLibrary.Conv_IntToDouble` (* _index_2 1000))) (struct)) false))))

(event `self.HierarchicalInstancedMesh.OnComponentBeginOverlap`
  (params (OverlappedComponent :type "PrimitiveComponent Object Reference") (OtherActor :type "Actor Object Reference") (OtherComp :type "PrimitiveComponent Object Reference") (OtherBodyIndex :type Integer) (bFromSweep :type Boolean) (SweepResult :type "HitResult Structure (by ref)"))
  (bind _hierarchicalinstancedmesh (`self.HierarchicalInstancedMesh`))
  (cast `/Game/MazeGame/Characters/MGHero/BP_MGHeroCharacter` OtherActor)
  (`InstancedStaticMeshComponent.RemoveInstance` _hierarchicalinstancedmesh (`|GetArrayItem` (`InstancedStaticMeshComponent.GetInstancesOverlappingSphere` _hierarchicalinstancedmesh (`.ImpactPoint` (`GameplayStatics.BreakHitResult` SweepResult)) 10.0 true))))

(fn `UserConstructionScript`)