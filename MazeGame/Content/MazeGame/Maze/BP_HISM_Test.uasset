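; BP_HISM_Test is a test actor in the maze game folder that fills a Hierarchical Instanced Static Mesh component with a flat grid of mesh instances.
; On BeginPlay, two nested loops add evenly spaced, unrotated, unit-scale instances along X and Y.
; The construction script is empty, and an instance-count debug print is left unconnected.
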(event `self.ReceiveBeginPlay`
  (for _index (range 6)
    (for _index_2 (range 6)
      (`InstancedStaticMeshComponent.AddInstance` (`self.HierarchicalInstancedStaticMesh`) (`KismetMathLibrary.MakeTransform` (`KismetMathLibrary.MakeVector` (`KismetMathLibrary.Conv_IntToDouble` (* _index_2 150)) (`KismetMathLibrary.Conv_IntToDouble` (* _index 150))))))))

(fn `UserConstructionScript`)