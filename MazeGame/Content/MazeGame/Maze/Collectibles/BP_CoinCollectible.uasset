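; BP_CoinCollectible is a coin pickup for the maze game that grants coins to the hero character on overlap.
; On overlap with BP_MGHeroCharacter, it applies GE_AddCoins through the hero's Ability System Component, passing CoinsToAdd as a SetByCaller magnitude, then destroys itself.
; The construction script applies a small random roll and pitch so placed coins look varied.
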(event `self.ReceiveActorBeginOverlap`
  (params (OtherActor :type "Actor Object Reference"))
  (bind _asbp_mghero_character (cast `/Game/MazeGame/Characters/MGHero/BP_MGHeroCharacter` OtherActor))
  (bind _returnvalue (`AbilitySystemBlueprintLibrary.GetAbilitySystemComponent` _asbp_mghero_character))
  (bind _returnvalue_2 (`AbilitySystemBlueprintLibrary.AssignTagSetByCallerMagnitude` (`AbilitySystemComponent.MakeOutgoingSpec` :`self` _returnvalue :`GameplayEffectClass` "/Game/MazeGame/Characters/MGHero/GamepalyEffects/GE_AddCoins.GE_AddCoins_C" :`Level` 1.0) (struct :`TagName` "SetByCaller.Coins") (`self.CoinsToAdd`)))
  (`AbilitySystemComponent.BP_ApplyGameplayEffectSpecToSelf` _returnvalue _returnvalue_2)
  (`self.K2_DestroyActor`))

(fn `UserConstructionScript`
  (`self.K2_SetActorRotation` (`KismetMathLibrary.MakeRotator` (`KismetMathLibrary.RandomFloatInRange` -10.0 10.0) (`KismetMathLibrary.RandomFloatInRange` -10.0 10.0))))