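; BP_EnergyCollectibleHISMFull is a maze collectible that grants the hero an energy amount equal to its maximum.
; All pickups are instances of one HierarchicalInstancedMesh, whose overlap event accepts only BP_MGHeroCharacter.
; A sphere query at the sweep impact point identifies the touched instance and removes it, printing an error if none is found.
; GE_AddEnergy is then applied through GAS with a SetByCaller magnitude.
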(event `self.HierarchicalInstancedMesh.OnComponentBeginOverlap`
  (params (OverlappedComponent :type "PrimitiveComponent Object Reference") (OtherActor :type "Actor Object Reference") (OtherComp :type "PrimitiveComponent Object Reference") (OtherBodyIndex :type Integer) (bFromSweep :type Boolean) (SweepResult :type "HitResult Structure (by ref)"))
  (bind _hierarchicalinstancedmesh (`self.HierarchicalInstancedMesh`))
  (bind _returnvalue (`InstancedStaticMeshComponent.GetInstancesOverlappingSphere` _hierarchicalinstancedmesh (`.ImpactPoint` (`GameplayStatics.BreakHitResult` SweepResult)) 50.0 true))
  (bind _asbp_mghero_character (cast `/Game/MazeGame/Characters/MGHero/BP_MGHeroCharacter` OtherActor))
  (if (not (`KismetArrayLibrary.Array_IsValidIndex` _returnvalue))
    (`KismetSystemLibrary.PrintString` "ERROR EMPTY OVERLAP"))
  (`InstancedStaticMeshComponent.RemoveInstance` _hierarchicalinstancedmesh (`|GetArrayItem` _returnvalue))
  (bind _returnvalue_2 (`AbilitySystemBlueprintLibrary.GetAbilitySystemComponent` _asbp_mghero_character))
  (bind _returnvalue_3 (`AbilitySystemBlueprintLibrary.AssignTagSetByCallerMagnitude` (`AbilitySystemComponent.MakeOutgoingSpec` :`self` _returnvalue_2 :`GameplayEffectClass` "/Game/MazeGame/Characters/MGHero/GamepalyEffects/GE_AddEnergy.GE_AddEnergy_C" :`Level` 1.0) (struct :`TagName` "SetByCaller.Energy") (`MGCharacterBase.GetMaxEnergy` _asbp_mghero_character)))
  (`AbilitySystemComponent.BP_ApplyGameplayEffectSpecToSelf` _returnvalue_2 _returnvalue_3))

(fn `UserConstructionScript`)