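; Coin collectible for the maze game that holds coins as hierarchical instanced mesh instances and awards coins to the hero on overlap.
; When a BP_MGHeroCharacter overlaps, it finds instances in a small sphere at the sweep impact point and removes the first.
; It then applies GE_AddCoins through the hero's Ability System Component, passing CoinsToAdd as a SetByCaller magnitude.
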(event `self.HierarchicalInstancedMesh.OnComponentBeginOverlap`
  (params (OverlappedComponent :type "PrimitiveComponent Object Reference") (OtherActor :type "Actor Object Reference") (OtherComp :type "PrimitiveComponent Object Reference") (OtherBodyIndex :type Integer) (bFromSweep :type Boolean) (SweepResult :type "HitResult Structure (by ref)"))
  (bind _hierarchicalinstancedmesh (`self.HierarchicalInstancedMesh`))
  (bind _asbp_mghero_character (cast `/Game/MazeGame/Characters/MGHero/BP_MGHeroCharacter` OtherActor))
  (`InstancedStaticMeshComponent.RemoveInstance` _hierarchicalinstancedmesh (`|GetArrayItem` (`InstancedStaticMeshComponent.GetInstancesOverlappingSphere` _hierarchicalinstancedmesh (`.ImpactPoint` (`GameplayStatics.BreakHitResult` SweepResult)) 10.0 true)))
  (bind _returnvalue (`AbilitySystemBlueprintLibrary.GetAbilitySystemComponent` _asbp_mghero_character))
  (bind _returnvalue_2 (`AbilitySystemBlueprintLibrary.AssignTagSetByCallerMagnitude` (`AbilitySystemComponent.MakeOutgoingSpec` :`self` _returnvalue :`GameplayEffectClass` "/Game/MazeGame/Characters/MGHero/GamepalyEffects/GE_AddCoins.GE_AddCoins_C" :`Level` 1.0) (struct :`TagName` "SetByCaller.Coins") (`self.CoinsToAdd`)))
  (`AbilitySystemComponent.BP_ApplyGameplayEffectSpecToSelf` _returnvalue _returnvalue_2))

(fn `UserConstructionScript`)