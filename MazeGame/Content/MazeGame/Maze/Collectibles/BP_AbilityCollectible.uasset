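; Maze pickup that unlocks a random, still-locked ability when the hero character overlaps its widget component.
; On BeginPlay it shuffles the save's ability levels, picks a level-zero key absent from the spawned-collectibles cache and reserves it there, preventing duplicates.
; It shows that ability's image widget, or destroys itself if none qualifies.
; Pickup sets the ability to level one in both save arrays, then destroys the actor.
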(event `self.ReceiveBeginPlay`
  (bind _abilitykey (`self.GetAbilityKey`))
  (bind _output_get (set `self.AbilityKey` _abilitykey))
  (if (`KismetStringLibrary.IsEmpty` _output_get)
    (`self.K2_DestroyActor`)
    (else
      (bind _returnvalue (`|CreateWidget` "/Game/MazeGame/UI/Widgets/3D/WBP_AbilityImage.WBP_AbilityImage_C" null (`self.AbilityKey`)))
      (`WidgetComponent.SetWidget` (`self.Widget`) _returnvalue))))

(event `self.Widget.OnComponentBeginOverlap`
  (params (OverlappedComponent :type "PrimitiveComponent Object Reference") (OtherActor :type "Actor Object Reference") (OtherComp :type "PrimitiveComponent Object Reference") (OtherBodyIndex :type Integer) (bFromSweep :type Boolean) (SweepResult :type "HitResult Structure (by ref)"))
  (bind _abilitykey (`self.AbilityKey`))
  (bind _abilitykey_2 (`self.AbilityKey`))
  (bind _currentlyloadedsavegameobject (`MGPlayerDataSubsystem.CurrentlyLoadedSaveGameObject` (subsystem `MGPlayerDataSubsystem`)))
  (bind _abilitieslevels (`MGSaveGame.AbilitiesLevels` _currentlyloadedsavegameobject))
  (bind _spawnedabilitycollectiblescache (`MGSaveGame.SpawnedAbilityCollectiblesCache` _currentlyloadedsavegameobject))
  (cast `/Game/MazeGame/Characters/MGHero/BP_MGHeroCharacter` OtherActor)
  (for (_array_element _array_index) _abilitieslevels
    (if (`KismetStringLibrary.EqualEqual_StrStr` (`.AbilityKey` (break `SavedAbilityInfo` _array_element)) _abilitykey)
      (`KismetArrayLibrary.Array_Set` _abilitieslevels _array_index (make `SavedAbilityInfo` _abilitykey 1))
      (for (_array_element_2 _array_index_2) _spawnedabilitycollectiblescache
        (if (`KismetStringLibrary.EqualEqual_StrStr` (`.AbilityKey` (break `SavedAbilityInfo` _array_element_2)) _abilitykey_2)
          (`KismetArrayLibrary.Array_Set` _spawnedabilitycollectiblescache _array_index_2 (make `SavedAbilityInfo` _abilitykey_2 1))
          (break)))
      (break)))
  (`self.K2_DestroyActor`))

(fn `GetAbilityKey`
  (returns (AbilityKey :type String))
  (locals (AbilitiesLevelsCache :type "Array of SavedAbilityInfo Structure") (Contains :type Boolean))
  (bind _currentlyloadedsavegameobject (`MGPlayerDataSubsystem.CurrentlyLoadedSaveGameObject` (subsystem `MGPlayerDataSubsystem`)))
  (bind _spawnedabilitycollectiblescache (`MGSaveGame.SpawnedAbilityCollectiblesCache` _currentlyloadedsavegameobject))
  (bind _output_get (set `local.AbilitiesLevelsCache` (`MGSaveGame.AbilitiesLevels` _currentlyloadedsavegameobject)))
  (`KismetArrayLibrary.Array_Shuffle` _output_get)
  (for _array_element (`local.AbilitiesLevelsCache`)
    (set `local.Contains` false)
    (for _array_element_2 _spawnedabilitycollectiblescache
      (bind (_abilitykey _abilityinfo) (break `SavedAbilityInfo` _array_element))
      (if (`KismetStringLibrary.EqualEqual_StrStr` _abilitykey (`.AbilityKey` (break `SavedAbilityInfo` _array_element_2)))
        (set `local.Contains` true)))
    (if (and (== _abilityinfo 0) (not (`local.Contains`)))
      (`KismetArrayLibrary.Array_Add` _spawnedabilitycollectiblescache (make `SavedAbilityInfo` _abilitykey))
      (return _abilitykey)))
  (return ""))

(fn `UserConstructionScript`)